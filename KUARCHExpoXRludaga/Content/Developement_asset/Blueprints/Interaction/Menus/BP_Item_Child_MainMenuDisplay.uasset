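; Main menu display item built on the interaction item template, set to stay in place with an inactive base, so it can only be manipulated.
; CustomizeSubcomponents spawns a BP_ManSCLogic for one button subcomponent and registers it in SubComponentMap as an anchor that can attach to "magwell" tags.
; Hang search sphere-traces from attach points for matching tagged components.
; Activation logic is mostly template test code: a base material swap with auto-reset and empty subcomponent branches.
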(event EventBeginPlay
  (bind _primaryghosthand (Variables|Default|GetPrimaryGhostHand))
  (bind _returnvalue (Transformation|GetRelativeTransform _primaryghosthand))
  ;[1 1 1] Start
  (|CallParentFunction)
  ;[1 0.2679 0] Customize Item Here
  (Utilities|FlowControl|Sequence
    (:then_0
      ;[1 0.7633 0] Determine placement in hand when gripped
      (Variables|Default|SetHandOffset (Math|Transform|MakeTransform (.location _returnvalue) (.rotation _returnvalue) "1,1,1"))
      ;[1 1 1] The green and blue arrows both fall along this axis
      (Variables|Default|SetReflectionAxis (Utilities|Enum|LiteralenumAxisEnum "NewEnumerator0"))
      ;[1 1 1] Hand pose when gripped
      (Variables|Default|SetGripType "NewEnumerator3")
      (Variables|Default|SetGripOverride 0.8))
    (:then_1
      ;[1 0.7388 0] Item Dropped only on second grip start
      (Variables|Default|SetSticky? false)
      ;[1 0.75 0] Item cannot be picked up, only manipulated/activated
      (Variables|Default|SetStayPut? true)
      ;[1 0.75 0] Base Item is Inactive
      (Variables|Default|SetDummy? true)
      ;[1 0.8032 0] Look for hang targets on tick or only on drop?
      (Variables|Default|SetSearchHangConstant? false)
      ;[1 0.9595 0] Hang on valid targets only when dropped, or as soon as acquired?
      (Variables|Default|SetHangDropOnly? true))
    (:then_2
      (Utilities|FlowControl|Sequence))))

(event EventTick
  (params (DeltaSeconds :type Float%20%28single-precision%29))
  ;[1 1 1] Tick
  (|CallParentFunction DeltaSeconds))

(event Custom|CheckActivation
  (Utilities|FlowControl|Sequence
    (:then_0
      ;[1 1 1] Activation state of the base item
      (if (Variables|Default|GetActivated?)
        ;[1 0.4875 0] Default Base Item Activation for Testing
        (CallFunction|ActivateBaseItem)
        (Utilities|AutoBaseDeactivate 0.1)
        (else
          (CallFunction|DeactivateBaseItem))))
    (:then_1
      ;[1 1 1] Manually Cycle through SubComponents
      (Utilities|FlowControl|Sequence
        (:then_0
          ;[1 0.4875 0] Default SubComponent Activation for Testing
          (bind _struct (Utilities|SubActivityBranch)))
        (:then_1
          (bind _struct_2 (Utilities|SubActivityBranch 1)))))))

(fn ConstructionScript
  (|CallParentFunction))

(fn ActiveComponentActions
  (params (TargetComponent :type Scene%20Component%20Object%20Reference) (Activated? :type Boolean))
  (switch int 0))

(fn ActiveItemActions
  (params (Activated? :type Boolean))
  (|CallParentFunction false))

(fn ManipulatedComponentActions
  (params (Component%20Struct :type Struct%20Item%20Sub%20Comp%20Properties%20Structure%20%28by%20ref%29)))

(fn CustomizeSubcomponents
  (bind _man0scene (Variables|Default|GetMan0Scene))
  (bind _man0mesh (Variables|Default|GetMan0Mesh))
  (bind _man0highlighter (Variables|Default|GetMan0Highlighter))
  ;[1 1 1] SetupManComps
  (Utilities|FlowControl|Sequence
    (:then_0
      ;[1 1 1] All the Sub Component-specific variables and logic live here
      (bind _returnvalue (Game|SpawnActorfromClass "/Game/Blueprints/Interaction/BP_ManSCLogic.BP_ManSCLogic_C" (Transformation|GetActorTransform) "AlwaysSpawn" 0 self "0.000000,0.000000,0.000000" (Utilities|Array|MakeArray (Transformation|GetRelativeTransform _man0scene)) _man0mesh "0.000000,0.000000,0.000000" (Variables|Default|GetMan0HandGhost) false _man0scene true false (Utilities|Struct|MakeStruct_ConstraintContainer "NewEnumerator1" (Utilities|Struct|MakeStruct_ButtonConstraints false false -1e+01 1e+01 0.0 0.0 0.0 0.0 3e+01) (Utilities|Struct|MakeStruct_LinearConstraints "NewEnumerator0" 0.0) (Utilities|Struct|MakeStruct_LinearConstraints "NewEnumerator0" 0.0) (Utilities|Struct|MakeStruct_LinearConstraints "NewEnumerator0" 0.0 25.0 1e+02) (Utilities|Struct|MakeStruct_AngularConstraints "NewEnumerator0" 0.0) (Utilities|Struct|MakeStruct_AngularConstraints "NewEnumerator0" 0.0 0.0 0.0 "NewEnumerator0") (Utilities|Struct|MakeStruct_AngularConstraints "NewEnumerator0" 0.0 0.0 0.0 "NewEnumerator2") (Utilities|Struct|MakeStruct_RadialConstraints false "NewEnumerator2")) _man0highlighter "NewEnumerator1" 1.0 true false 0))
      ;[1 1 1] For Use by Item BP
      (Utilities|Map|Add (Variables|Default|GetSubComponentMap) _man0mesh (Utilities|Struct|MakeStruct_ItemSubCompProperties _man0mesh _man0scene _man0highlighter _returnvalue (Utilities|Struct|MakeMaleAttacherStruct true (Utilities|Array|MakeArray "magwell") (Variables|Default|GetAttach0Ref)) (Utilities|Struct|MakeFemaleAttacherStruct false "(\"\")" 0 false) false true)))))

(fn ActivateBaseItem
  (Rendering|Material|SetMaterial (Variables|Default|GetBaseMesh) 0 "/Engine/VREditor/BasicMeshes/MI_Cube_02.MI_Cube_02"))

(fn DeactivateBaseItem
  (Rendering|Material|SetMaterial (Variables|Default|GetBaseMesh) 0 "/Engine/VREditor/BasicMeshes/MI_Cube_01.MI_Cube_01"))

(fn SearchHangTarget0
  (Variables|Default|SetHangTarget 0)
  (Variables|Default|SetHangTargetActor 0)
  (Variables|Default|SetAttachingScene 0)
  (LocalVariables|SetTargetFemaleComponent 0)
  (bind _array_element (Utilities|Array|ForEachLoopwithBreak (Variables|Default|GetSubComponentArray))
    (:LoopBody
      (if (.MaleAttachable? (Utilities|Struct|BreakMaleAttacherStruct (.MaleAttachments (Utilities|Struct|BreakStruct_ItemSubCompProperties _array_element))))
        (bind (_outhits _returnvalue) (Collision|MultiSphereTraceForObjects (Transformation|GetWorldLocation (.MaleAttachLocationRefScene (Utilities|Struct|BreakMaleAttacherStruct (.MaleAttachments (Utilities|Struct|BreakStruct_ItemSubCompProperties _array_element))))) (Transformation|GetWorldLocation (.MaleAttachLocationRefScene (Utilities|Struct|BreakMaleAttacherStruct (.MaleAttachments (Utilities|Struct|BreakStruct_ItemSubCompProperties _array_element))))) 5.0 (Utilities|Array|MakeArray "ObjectTypeQuery1" "ObjectTypeQuery2" "ObjectTypeQuery3" "ObjectTypeQuery4") false 0 "None"))
        (if _returnvalue
          (for _array_element_2 _outhits
            (for _array_element_3 (.TagTargets (Utilities|Struct|BreakMaleAttacherStruct (.MaleAttachments (Utilities|Struct|BreakStruct_ItemSubCompProperties _array_element))))
              (if (Utilities|Array|ContainsItem (Variables|/Script/Engine.ActorComponent|GetComponentTags (.HitComponent (Collision|BreakHitResult _array_element_2))) _array_element_3)
                (bind _asbp_item_base (Utilities|Casting|CastToBP_Item_Base (.HitActor (Collision|BreakHitResult _array_element_2)))
                  (:then
                    (if (.ReturnValue (Utilities|Map|Find (Variables|/Game/Blueprints/Interaction/BP_Item_Base.BP_Item_Base_C|GetSubComponentMap _asbp_item_base) (.HitComponent (Collision|BreakHitResult _array_element_2))))
                      (if (.AttachedNow? (Utilities|Struct|BreakFemaleAttacherStruct (.FemaleAttachments (Utilities|Struct|BreakStruct_ItemSubCompProperties (.Value (Utilities|Map|Find (Variables|/Game/Blueprints/Interaction/BP_Item_Base.BP_Item_Base_C|GetSubComponentMap _asbp_item_base) (.HitComponent (Collision|BreakHitResult _array_element_2))))))))
                        (Variables|Default|SetHangTarget 0 :!label _label)
                        (Variables|Default|SetAttachingScene 0)
                        (LocalVariables|SetTargetFemaleComponent 0)
                        (Variables|Default|SetHangTargetActor 0)
                        (else
                          (LocalVariables|SetTargetFemaleComponent (.FemaleAttachLocationRefScene (Utilities|Struct|BreakFemaleAttacherStruct (.FemaleAttachments (Utilities|Struct|BreakStruct_ItemSubCompProperties (.Value (Utilities|Map|Find (Variables|/Game/Blueprints/Interaction/BP_Item_Base.BP_Item_Base_C|GetSubComponentMap _asbp_item_base) (.HitComponent (Collision|BreakHitResult _array_element_2)))))))))
                          (LocalVariables|SetHangActor (.HitActor (Collision|BreakHitResult _array_element_2)))))
                      (else
                        (LocalVariables|SetTargetFemaleComponent (.HitComponent (Collision|BreakHitResult _array_element_2)) :!label _label_2))))
                  (:CastFailed
                    (goto _label_2)))
                (else
                  (goto _label)))
              (return (LocalVariables|GetTargetFemaleComponent) (.MaleAttachLocationRefScene (Utilities|Struct|BreakMaleAttacherStruct (.MaleAttachments (Utilities|Struct|BreakStruct_ItemSubCompProperties _array_element)))) (LocalVariables|GetHangActor))))
          (else
            (Variables|Default|SetHangTarget 0)
            (Variables|Default|SetAttachingScene 0)
            (LocalVariables|SetTargetFemaleComponent 0)
            (Variables|Default|SetHangTargetActor 0)
            (return (LocalVariables|GetTargetFemaleComponent) (.MaleAttachLocationRefScene (Utilities|Struct|BreakMaleAttacherStruct (.MaleAttachments (Utilities|Struct|BreakStruct_ItemSubCompProperties _array_element)))) (LocalVariables|GetHangActor))))))))

(fn HangPreview)