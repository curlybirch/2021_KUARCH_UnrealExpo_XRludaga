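; Prototype dummy interaction item that serves as a moving anchor, stay-put so it can be manipulated but not picked up.
; BeginPlay sets grip settings and spawns BP_ManSCLogic for one constrained manipulable sub-component, registered as an anchor in SubComponentMap.
; Tick bobs the whole actor vertically by a fixed per-frame offset, using a Delay to flip direction about every three seconds, so travel depends on frame rate.
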(event EventBeginPlay
  (bind _man0scene (Variables|Default|GetMan0Scene))
  (bind _man0mesh (Variables|Default|GetMan0Mesh))
  (bind _man0highlighter (Variables|Default|GetMan0Highlighter))
  (bind _primaryghosthand (Variables|Default|GetPrimaryGhostHand))
  (bind _returnvalue (Transformation|GetRelativeTransform _primaryghosthand))
  (|CallParentFunction)
  (Utilities|FlowControl|Sequence
    (:then_0
      ;[1 0.2679 0] Customize Item Here
      (Utilities|FlowControl|Sequence
        (:then_0
          ;[1 0.7633 0] Determine placement in hand when gripped
          (Variables|Default|SetHandOffset (Math|Transform|MakeTransform (.location _returnvalue) (.rotation _returnvalue) "1,1,1"))
          ;[1 1 1] The green and blue arrows both fall along this axis
          (Variables|Default|SetReflectionAxis (Utilities|Enum|LiteralenumAxisEnum "NewEnumerator0"))
          ;[1 1 1] Hand pose when gripped
          (Variables|Default|SetGripType "NewEnumerator3")
          (Variables|Default|SetGripOverride 0.8))
        (:then_1
          ;[1 0.7388 0] Item Dropped only on second grip start
          (Variables|Default|SetSticky? false)
          ;[1 0.75 0] Item cannot be picked up, only manipulated/activated
          (Variables|Default|SetStayPut? true)
          ;[1 0.75 0] Base Item is Inactive
          (Variables|Default|SetDummy? true)
          ;[1 0.8032 0] Look for hang targets on tick or only on drop?
          (Variables|Default|SetSearchHangConstant? false)
          ;[1 0.9595 0] Hang on valid targets only when dropped, or as soon as acquired?
          (Variables|Default|SetHangDropOnly? true))))
    (:then_1
      (Utilities|FlowControl|Sequence
        (:then_0
          ;[1 1 1] SetupManComps
          (Utilities|FlowControl|Sequence
            (:then_0
              ;[1 1 1] All the Sub Component-specific variables and logic live here
              (bind _returnvalue_2 (Game|SpawnActorfromClass "/Game/Blueprints/Interaction/BP_ManSCLogic.BP_ManSCLogic_C" (Transformation|GetActorTransform) "AlwaysSpawn" 0 self "0.000000,0.000000,0.000000" (Utilities|Array|MakeArray (Transformation|GetRelativeTransform _man0scene)) _man0mesh "0.000000,0.000000,0.000000" (Variables|Default|GetMan0HandGhost) true _man0scene true true (Utilities|Struct|MakeStruct_ConstraintContainer "NewEnumerator1" (Utilities|Struct|MakeStruct_ButtonConstraints false false -1e+01 1e+01) (Utilities|Struct|MakeStruct_LinearConstraints "NewEnumerator0" 0.0) (Utilities|Struct|MakeStruct_LinearConstraints "NewEnumerator0" 0.0) (Utilities|Struct|MakeStruct_LinearConstraints "NewEnumerator0" 0.0 25.0 1e+02) (Utilities|Struct|MakeStruct_AngularConstraints "NewEnumerator0" 0.0) (Utilities|Struct|MakeStruct_AngularConstraints "NewEnumerator0" 0.0 0.0 0.0 "NewEnumerator0") (Utilities|Struct|MakeStruct_AngularConstraints "NewEnumerator0" 0.0 0.0 0.0 "NewEnumerator2") (Utilities|Struct|MakeStruct_RadialConstraints false "NewEnumerator2")) _man0highlighter "NewEnumerator1" 1.0 false 0))
              ;[1 1 1] For Use by Item BP
              (Utilities|Map|Add (Variables|Default|GetSubComponentMap) _man0mesh (Utilities|Struct|MakeStruct_ItemSubCompProperties _man0mesh _man0scene _man0highlighter _returnvalue_2 (Utilities|Struct|MakeMaleAttacherStruct false (Utilities|Array|MakeArray "None")) (Utilities|Struct|MakeFemaleAttacherStruct false (Utilities|Array|MakeArray "None") 0 false) false true)))))
        (:then_1
          (bind _values (Utilities|Map|Values (Variables|Default|GetSubComponentMap)))
          (Variables|Default|SetSubComponentArray _values))))))

(event Collision|EventActorBeginOverlap
  (params (OtherActor :type Actor%20Object%20Reference)))

(event EventTick
  (params (DeltaSeconds :type Float%20%28single-precision%29))
  (|CallParentFunction DeltaSeconds)
  (Utilities|FlowControl|Sequence
    (:then_0
      (if (Variables|Default|GetUp?)
        (Transformation|AddActorWorldOffset "0, 0,0.100000")
        (else
          (Transformation|AddActorWorldOffset "0, 0,-0.100000"))))
    (:then_1
      (Utilities|FlowControl|Delay 3.0)
      (Variables|Default|SetUp? (not (Variables|Default|GetUp?))))))

(fn ConstructionScript
  (|CallParentFunction))

(fn CustomizeBaseItem
  (|CallParentFunction))