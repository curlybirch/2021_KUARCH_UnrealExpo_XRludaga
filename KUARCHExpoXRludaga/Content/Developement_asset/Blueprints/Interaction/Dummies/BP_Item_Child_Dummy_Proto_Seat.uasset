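; Prototype dummy item that acts as a seat a pawn can sit on, built as a child of an interaction item Blueprint.
; On BeginPlay it registers the Man0 scene, mesh, highlighter and ghost hand as a sub-component that is grabbable, an anchor and a seat, with a grip override.
; The seat attach event calls SitDown on the pawn, passing the Attach1 reference.
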(event EventBeginPlay
  (|CallParentFunction)
  (CallFunction|AddLogictoSubComponent :Scene (Variables|Default|GetMan0Scene) :Mesh (Variables|Default|GetMan0Mesh) :HighlightCap (Variables|Default|GetMan0Highlighter) :Ghosthand (Variables|Default|GetMan0HandGhost) :Grip (Utilities|Struct|MakeStruct_GripOverrides "NewEnumerator1" 1.0) :Options (Utilities|Struct|MakeStruct_SubOptions true false true true true) :Tags (Utilities|Array|MakeArray "None")))

(event Collision|EventActorBeginOverlap
  (params (OtherActor :type Actor%20Object%20Reference)))

(event EventTick
  (params (DeltaSeconds :type Float%20%28single-precision%29))
  (|CallParentFunction DeltaSeconds) ; This node is disabled and will not be called.\nDrag off pins to build functionality.
)

(event EventAttachPawnActortoSeat
  (params (PawnActor :type BP%20VR%20Pawn%20Object%20Reference))
  (Default|SitDown PawnActor (Variables|Default|GetAttach1Ref)))

(fn ConstructionScript
  (|CallParentFunction))