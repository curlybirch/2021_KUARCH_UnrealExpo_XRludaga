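; VR interaction component that makes an item's sub-part hand-manipulable or pressable as a button.
; On grab it snaps the hand mesh to a ghost hand, then each tick applies hand movement through per-axis linear, rotational and look-at radial constraints.
; It auto-releases when the hand strays too far, with optional position reset or pawn seating.
; Button mode follows the fingertip along clamped X, springs back unless sticky, and supports threshold-based toggling.
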(event Custom|OnManEnd
  (CallFunction|DetachHand)
  (CallFunction|ResetHand)
  (Default|HandChangeOverride (Variables|Default|GetManipulatingHand) "NewEnumerator0" 0.0)
  (Utilities|FlowControl|Sequence
    (:then_0
      (if (Variables|Default|GetSeat?)
        (Default|AttachPawnActortoSeat (Variables|Default|GetOwningItem) (.AsBP%20VR%20Pawn (Utilities|Casting|CastToBP_VR_Pawn (Variables|/Game/Blueprints/Pawn/BP_VR_Hand.BP_VR_Hand_C|GetOwningPawn (Variables|Default|GetManipulatingHand)))))))
    (:then_1
      (Variables|Default|SetManipulating false)
      (Variables|Default|SetManipulatingHand 0)
      (Variables|Default|SetRelativeZeroTrans "")
      ;[1 0 0] Fix by Axis
      (if (Variables|Default|GetResetPosOnDrop?)
        (CallFunction|ResetPosition)))))

(event Custom|OnManStart
  (params (ManHand :type BP%20VR%20Hand%20Object%20Reference))
  (bind _targetscenebase (Variables|Default|GetTargetSceneBase))
  (bind _relativerotation (Variables|/Script/Engine.SceneComponent|GetRelativeRotation _targetscenebase))
  (Utilities|IsValid ManHand
    (:Is%20Valid
      (Variables|Default|SetManipulatingHand ManHand)
      (Variables|Default|SetManipulating true)
      (CallFunction|AttachHandMeshtoComponent)
      (Variables|Default|SetInitialDistance (Math|Vector|Distance(Vector) (Transformation|GetActorLocation ManHand) (Transformation|GetWorldLocation (Variables|Default|GetTargetComponent))))
      (Variables|Default|SetInitialLocation (Variables|/Script/Engine.SceneComponent|GetRelativeLocation _targetscenebase))
      (Variables|Default|SetInitialRotation (Math|Vector|MakeVector (.roll _relativerotation) (.pitch _relativerotation) (.yaw _relativerotation)))
      (Variables|Default|SetRelativeZeroTrans (Utilities|GetRelativeTransHand-Comp))
      (Default|HandChangeOverride ManHand (Variables|Default|GetGripType) (Variables|Default|GetGripOverride)))))

(event Custom|HighlightComponent
  (bind _highlighter (Variables|Default|GetHighlighter))
  (if (Variables|/Game/Blueprints/Interaction/BP_Item_Base.BP_Item_Base_C|GetHeld? (Variables|Default|GetOwningItem))
    (Utilities|IsValid _highlighter
      (:Is%20Valid
        (Rendering|SetVisibility _highlighter true false)
        (Development|SetHiddeninGame _highlighter false false :!label _label)
        (Utilities|FlowControl|RetriggerableDelay 0.05)
        (Development|SetHiddeninGame _highlighter true false)))
    (elif (Variables|Default|GetCanManWOHold?)
      (goto _label)
      (else
        (Default|Highlight (Variables|Default|GetOwningItem))))))

(event EventBeginPlay
  ;[1 1 1] Start
  (Utilities|FlowControl|Sequence
    (:then_0
      (CallFunction|AttachSelftoItem))))

(event EventTick
  (params (DeltaSeconds :type Float%20%28single-precision%29))
  ;[1 1 1] Tick
  (Utilities|FlowControl|Sequence
    (:then_1
      (Utilities|FlowControl|Sequence
        (:then_0
          (if (Variables|Default|GetManipulating)
            (Utilities|FlowControl|Sequence
              (:then_0
                (CallFunction|DoMoveConstrained))
              (:then_1
                (CallFunction|HandDistanceCheck))
              (:then_2
                ;[1 0 0] Set relative constraints by testing rotation against subcomponent ghost hand.
                ;
                ; Make all this variable exposed on spawn
                (CallFunction|RotateHand "palmsock")))))
        (:then_1
          (if (Variables|Default|GetButton?)
            (Transformation|SetWorldLocation (Variables|Default|GetStayOnMesh) (Transformation|GetWorldLocation (Variables|Default|GetTargetComponent)) false false)
            (CallFunction|AmButton)))))))

(event Custom|DoMoveConstrained
  (bind _targetscenebase (Variables|Default|GetTargetSceneBase))
  (bind _targetscenebase_2 (Variables|Default|GetTargetSceneBase))
  (bind _relativerotation (Variables|/Script/Engine.SceneComponent|GetRelativeRotation _targetscenebase))
  (bind (_roll _pitch _yaw) (Math|Rotator|BreakRotator _relativerotation))
  (Utilities|FlowControl|Sequence
    (:then_0
      (switch Utilities|FlowControl|Switch|SwitchonRelEnum (.linearrelativespace (Variables|Default|GetMovementConstraints))
        (:NewEnumerator1
          (bind _newtargetpositemspace (Utilities|FindTargetItemSpace))
          (bind _constrainedtargetpos (Utilities|CalcNewPos (Variables|/Script/Engine.SceneComponent|GetRelativeLocation _targetscenebase_2) _newtargetpositemspace _targetscenebase_2)
            (:Completed
              (Transformation|SetRelativeLocation _targetscenebase_2 _constrainedtargetpos true false))))))
    (:then_1
      (bind _newtargetrotitemspace (Utilities|FindTargetItemSpace))
      (bind _constrainedtargetrot (Utilities|CalcNewRot (Math|Vector|MakeVector _roll _pitch _yaw) _newtargetrotitemspace _targetscenebase)
        (:Completed
          (Transformation|SetRelativeRotation _targetscenebase (Math|Rotator|MakeRotator (.x _constrainedtargetrot) (.y _constrainedtargetrot) (.z _constrainedtargetrot)) false false))))
    (:then_2
      (bind _newrad (Utilities|CalcNewRad)
        (:NewParam
          ;[1 0 0] Fix Ghost Hand Rotation
          (Transformation|SetRelativeRotation (.PolarOrigin (Utilities|Struct|BreakStruct_RadialConstraints (.Radial (Utilities|Struct|BreakStruct_ConstraintContainer (Variables|Default|GetMovementConstraints))))) (Math|Rotator|MakeRotator (.x _newrad) (.y _newrad) (.z _newrad)) false false))))))

(event Custom|DoButtonMove
  (CallFunction|ButtonMove))

(event Custom|ResetButton
  (if (Variables|Default|GetResetting?)
    (CallFunction|ResetMovement)))

(event Custom|AmButton
  (bind _movementconstraints (Variables|Default|GetMovementConstraints))
  (bind _movementconstraints_2 (Variables|Default|GetMovementConstraints))
  (bind _targetcomponent (Variables|Default|GetTargetComponent))
  (bind _button (Utilities|Struct|BreakStruct_ConstraintContainer _movementconstraints))
  (bind _button_2 (Utilities|Struct|BreakStruct_ConstraintContainer _movementconstraints_2))
  (bind _relativelocation (Variables|/Script/Engine.SceneComponent|GetRelativeLocation _targetcomponent))
  (Utilities|FlowControl|Sequence
    (:then_0
      (if (Variables|Default|GetButtonInteraction?)
        (CallFunction|DoButtonMove)
        (elif (not (.sticky? (.Button (Utilities|Struct|BreakStruct_ConstraintContainer (Variables|Default|GetMovementConstraints)))))
          (Utilities|FlowControl|Sequence
            (:then_0
              (Utilities|FlowControl|Delay 0.05)
              (Variables|Default|SetResetting? true))
            (:then_1
              (CallFunction|ResetButton))))))
    (:then_1
      (if (.toggleable? _button_2)
        (Utilities|FlowControl|Sequence
          (:then_1
            (if (Variables|Default|GetActivated?)
              (Utilities|FlowControl|Sequence
                (:then_0
                  (if (Math|Float|NearlyEqual(Float) (.x _relativelocation) (Variables|Default|GetCurrentResetX) 0.4)
                    (goto _label Reset)))
                (:then_1
                  (if (<= (.x _relativelocation) (.toggleoffthresh _button_2))
                    (Utilities|FlowControl|DoOnce true :!label _label
                      (:Completed
                        (Variables|Default|SetActivated? false))))))
              (else
                (Utilities|FlowControl|Sequence
                  (:then_0
                    (if (Math|Float|NearlyEqual(Float) (.x _relativelocation) (Variables|Default|GetCurrentResetX) 0.4)
                      (goto _label_2 Reset)))
                  (:then_1
                    (if (<= (.x _relativelocation) (.activetoggleonthresh _button_2))
                      (Utilities|FlowControl|DoOnce true :!label _label_2
                        (:Completed
                          (Variables|Default|SetActivated? true))))))))))
        (elif (<= (.x _relativelocation) (.activetoggleonthresh _button_2))
          (Variables|Default|SetActivated? true)
          (else
            (Variables|Default|SetActivated? false)))))
    (:then_2
      (if (.toggleable? _button)
        (Utilities|FlowControl|Sequence
          (:then_0
            (if (Variables|Default|GetActivated?)
              (Variables|Default|SetCurrentResetX (.togglex _button))
              (else
                (Variables|Default|SetCurrentResetX (.resetx _button)))))
          (:then_1
            ;[0.9301 0 1] Debug
            (if (Variables|Default|GetActivated?) :!label _label_3
              (Rendering|Material|SetMaterial (.AsStatic%20Mesh%20Component (Utilities|Casting|CastToStaticMeshComponent (Variables|Default|GetTargetComponent))) 0 "/Engine/VREditor/BasicMeshes/MI_Cube_02.MI_Cube_02")
              (else
                (Rendering|Material|SetMaterial (.AsStatic%20Mesh%20Component (Utilities|Casting|CastToStaticMeshComponent (Variables|Default|GetTargetComponent))) 0 "/Engine/VREditor/BasicMeshes/MI_Cube_03.MI_Cube_03")))))
        (else
          (Variables|Default|SetCurrentResetX (.resetx _button))
          (goto _label_3))))))

(event Custom|ButtonFinger
  (params (PointerTipLocation :type Vector))
  (Variables|Default|SetPointerTipLocation PointerTipLocation)
  (Variables|Default|SetButtonInteraction? true)
  (Utilities|FlowControl|RetriggerableDelay 0.01)
  (Variables|Default|SetButtonInteraction? false)
  (Variables|Default|SetPointerTipLocation "0, 0, 0"))

(fn ConstructionScript)

(fn AttachHandMeshtoComponent
  (bind _manipulatinghand (Variables|Default|GetManipulatingHand))
  (bind _handmesh (Variables|/Game/Blueprints/Pawn/BP_VR_Hand.BP_VR_Hand_C|GetHandMesh _manipulatinghand))
  (Variables|/Game/Blueprints/Pawn/BP_VR_Hand.BP_VR_Hand_C|SetManipulatedActor _manipulatinghand (Variables|Default|GetOwningItem))
  (Variables|/Game/Blueprints/Pawn/BP_VR_Hand.BP_VR_Hand_C|SetManipulatedComponent _manipulatinghand (Variables|Default|GetTargetComponent))
  (Variables|/Game/Blueprints/Pawn/BP_VR_Hand.BP_VR_Hand_C|SetManipulating _manipulatinghand true)
  (Transformation|AttachComponentToComponent _handmesh (Variables|Default|GetGhostHand) "None" "SnapToTarget" "SnapToTarget" "KeepWorld" true)
  (if (not (Variables|/Game/Blueprints/Pawn/BP_VR_Hand.BP_VR_Hand_C|GetLeft0Rght1 _manipulatinghand))
    (Transformation|AddRelativeRotation _handmesh "0, 0,180.000000" false false)))

(fn AttachSubComponenttoLogicScene)

(fn MovementBoundsCheck)

(fn ResetPosition
  (bind _resetpositions (Variables|Default|GetResetPositions))
  (bind _resetkey (Variables|Default|GetResetKey))
  (bind _output (Utilities|Array|Get(acopy) _resetpositions _resetkey))
  (Transformation|SetRelativeLocationAndRotation (Variables|Default|GetTargetSceneBase) (.location _output) (.rotation _output) false false))

(fn SelectResetPosition)

(fn HandDistanceCheck
  (if (>= (Math|Vector|Distance(Vector) (Transformation|GetActorLocation (Variables|Default|GetManipulatingHand)) (Transformation|GetWorldLocation (Variables|Default|GetTargetComponent))) (* (Variables|Default|GetInitialDistance) 2.0))
    (CallFunction|OnManEnd)))

(fn MatchMotionControllerConstrained)

(fn DetachHand
  (bind _manipulatinghand (Variables|Default|GetManipulatingHand))
  (Default|AnchorGripped _manipulatinghand (Utilities|Struct|MakeStruct_ItemSubCompProperties) true)
  (Transformation|DetachFromComponent (Variables|/Game/Blueprints/Pawn/BP_VR_Hand.BP_VR_Hand_C|GetHandMesh _manipulatinghand) "KeepWorld" "KeepWorld" "KeepWorld" true)
  (Variables|/Game/Blueprints/Pawn/BP_VR_Hand.BP_VR_Hand_C|SetManipulatedActor _manipulatinghand (Variables|Default|GetOwningItem))
  (Variables|/Game/Blueprints/Pawn/BP_VR_Hand.BP_VR_Hand_C|SetManipulatedComponent _manipulatinghand (Variables|Default|GetTargetComponent))
  (Variables|/Game/Blueprints/Pawn/BP_VR_Hand.BP_VR_Hand_C|SetManipulating _manipulatinghand false))

(fn ResetHand
  (Default|ResetMeshLocation (Variables|Default|GetManipulatingHand)))

(fn AttachSelftoItem
  (Transformation|AttachComponentToComponent (Variables|Default|GetTargetSceneBase) "None" "SnapToTarget" "SnapToTarget" "KeepWorld" true))

(fn OLDMovement
  (Transformation|SetRelativeLocation (Variables|Default|GetTargetSceneBase) (+ (* (- (.location (Utilities|GetRelativeTransHand-Comp)) (.location (Variables|Default|GetRelativeZeroTrans))) (.x (Variables|/Script/Engine.SceneComponent|GetRelativeScale3D (Variables|Default|GetTargetSceneBase)))) (Variables|Default|GetInitialLocation)) false false))

(fn CalcConstrainedPosbyAxis
  (params (Struct_LinearConstraints :type Struct%20Linear%20Constraints%20Structure%20%28by%20ref%29) (Current :type Float%20%28single-precision%29) (Target :type Float%20%28single-precision%29))
  (bind (_boundstype _lockspecifiedvalue _min _max) (Utilities|Struct|BreakStruct_LinearConstraints Struct_LinearConstraints))
  (Utilities|FlowControl|Sequence
    (:then_0
      (switch Utilities|FlowControl|Switch|SwitchonConstraintEnum _boundstype
        (:NewEnumerator0
          (LocalVariables|SetPos1 Current))
        (:NewEnumerator1
          (LocalVariables|SetPos1 _lockspecifiedvalue))
        (:NewEnumerator2
          (LocalVariables|SetPos1 Target))
        (:NewEnumerator3
          (LocalVariables|SetPos1 (Math|Float|Clamp(Float) Target _min _max)))))
    (:then_1
      (return (LocalVariables|GetPos1)))))

(fn RotateHand
  (params (HandAttSock :type Name :default "palmsock"))
  (bind _manipulatinghand (Variables|Default|GetManipulatingHand))
  (bind _handmesh (Variables|/Game/Blueprints/Pawn/BP_VR_Hand.BP_VR_Hand_C|GetHandMesh _manipulatinghand))
  (bind _pawnghosthand (Variables|/Game/Blueprints/Pawn/BP_VR_Hand.BP_VR_Hand_C|GetPawnGhostHand _manipulatinghand))
  (Utilities|IsValid _manipulatinghand
    (:Is%20Valid
      (Utilities|IsValid _pawnghosthand
        (:Is%20Valid
          (Transformation|SetWorldRotation _handmesh (Transformation|GetWorldRotation _pawnghosthand) false false)
          (Transformation|SetWorldLocation _handmesh (+ (Transformation|GetSocketLocation (Variables|Default|GetGhostHand) HandAttSock) (- (Transformation|GetWorldLocation _pawnghosthand) (Transformation|GetSocketLocation _pawnghosthand HandAttSock))) false false))))))

(fn ButtonDetect
  (for _array_element (Class|PrimitiveComponent|GetOverlappingComponents (.AsPrimitive%20Component (Utilities|Casting|CastToPrimitiveComponent (Variables|Default|GetTargetComponent))))
    (if (Components|ComponentHasTag _array_element "pointertip")
      (Variables|Default|SetPointerTipLocation (Transformation|GetWorldLocation _array_element))
      (Variables|Default|SetButtonInteraction? true)
      (return)))
  (Variables|Default|SetButtonInteraction? false))

(fn ButtonMove
  (bind _movementconstraints (Variables|Default|GetMovementConstraints))
  (bind _sphere (Variables|Default|GetSphere))
  (bind _button (Utilities|Struct|BreakStruct_ConstraintContainer _movementconstraints))
  (bind _relativelocation (Variables|/Script/Engine.SceneComponent|GetRelativeLocation _sphere))
  (bind (_toggleable_ _sticky_ _minx _maxx) (Utilities|Struct|BreakStruct_ButtonConstraints _button))
  (LocalVariables|SetRefLocation (Variables|/Script/Engine.SceneComponent|GetRelativeLocation (Variables|Default|GetStayOnMesh)))
  ;[1 1 1] Match Finger
  (Transformation|SetWorldLocation (Variables|Default|GetSphere) (Variables|Default|GetPointerTipLocation) false false)
  (if (not (> (.x _relativelocation) (.x (Variables|/Script/Engine.SceneComponent|GetRelativeLocation (Variables|Default|GetStayOnMesh)))))
    (bind _output_get (LocalVariables|SetNewX (Math|Float|Clamp(Float) (.x _relativelocation) _minx _maxx)))
    (Transformation|SetRelativeLocation (Variables|Default|GetSphere) (Math|Vector|MakeVector _output_get (.y (LocalVariables|GetRefLocation)) (.z (LocalVariables|GetRefLocation))) false false)
    (Transformation|SetWorldLocation (Variables|Default|GetTargetComponent) (Transformation|GetWorldLocation (Variables|Default|GetSphere)) false false)))

(fn ResetMovement
  (bind _returnvalue (Utilities|Time|GetWorldDeltaSeconds))
  (bind _currentresetx (Variables|Default|GetCurrentResetX))
  (bind _movementconstraints (Variables|Default|GetMovementConstraints))
  (bind _targetcomponent (Variables|Default|GetTargetComponent))
  (bind _button (Utilities|Struct|BreakStruct_ConstraintContainer _movementconstraints))
  (bind _relativelocation (Variables|/Script/Engine.SceneComponent|GetRelativeLocation _targetcomponent))
  (bind _speed (Utilities|Struct|BreakStruct_ButtonConstraints _button))
  (bind _returnvalue_2 (* _speed _returnvalue))
  (if (not (Math|Float|NearlyEqual(Float) (.x _relativelocation) _currentresetx 0.1))
    (if (> (.x _relativelocation) _currentresetx)
      (Transformation|AddLocalOffset _targetcomponent (Math|Vector|MakeVector (* _returnvalue_2 -1.0) 0.0 0.0) false false)
      (elif (< (.x _relativelocation) _currentresetx)
        (Transformation|AddLocalOffset _targetcomponent (Math|Vector|MakeVector _returnvalue_2 0.0 0.0) false false)))))