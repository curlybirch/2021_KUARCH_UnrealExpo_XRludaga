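; Crossroad interaction actor that tilts four components, named by side and angle (right 30°/40°, left 70°/30°), while something overlaps its collision volume.
; Begin overlap plays one timeline whose separate tracks set each component's relative pitch, with the left pair held at 180° yaw.
; End overlap reverses the timeline; neither event filters which actor triggers it.
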(event OnComponentBeginOverlap(콜리전)
  (params (OverlappedComponent :type Primitive%20Component%20Object%20Reference) (OtherActor :type Actor%20Object%20Reference) (OtherComp :type Primitive%20Component%20Object%20Reference) (OtherBodyIndex :type Integer) (bFromSweep :type Boolean) (SweepResult :type Hit%20Result%20Structure%20%28by%20ref%29))
  (bind (_direction _왼쪽70도 _왼쪽30도 _오른쪽40도 _오른쪽30도) (Timeline|타임라인_0 Play)
    (:Update
      (Utilities|FlowControl|Sequence
        (:then_0
          (Transformation|SetRelativeRotation (Variables|Default|Get오른쪽30도) (Math|Rotator|MakeRotator 0.0 _오른쪽30도 0.0) false false))
        (:then_1
          (Transformation|SetRelativeRotation (Variables|Default|Get오른쪽40도) (Math|Rotator|MakeRotator 0.0 _오른쪽40도 0.0) false false))
        (:then_2
          (Transformation|SetRelativeRotation (Variables|Default|Get왼쪽70도) (Math|Rotator|MakeRotator 0.0 _왼쪽70도 1.8e+02) false false))
        (:then_3
          (Transformation|SetRelativeRotation (Variables|Default|Get왼쪽30도) (Math|Rotator|MakeRotator 0.0 _왼쪽30도 1.8e+02) false false))))))

(event OnComponentEndOverlap(콜리전)
  (params (OverlappedComponent :type Primitive%20Component%20Object%20Reference) (OtherActor :type Actor%20Object%20Reference) (OtherComp :type Primitive%20Component%20Object%20Reference) (OtherBodyIndex :type Integer))
  (bind (_direction _왼쪽70도 _왼쪽30도 _오른쪽40도 _오른쪽30도) (Timeline|타임라인_0 Reverse)
    (:Update
      (Utilities|FlowControl|Sequence
        (:then_0
          (Transformation|SetRelativeRotation (Variables|Default|Get오른쪽30도) (Math|Rotator|MakeRotator 0.0 _오른쪽30도 0.0) false false))
        (:then_1
          (Transformation|SetRelativeRotation (Variables|Default|Get오른쪽40도) (Math|Rotator|MakeRotator 0.0 _오른쪽40도 0.0) false false))
        (:then_2
          (Transformation|SetRelativeRotation (Variables|Default|Get왼쪽70도) (Math|Rotator|MakeRotator 0.0 _왼쪽70도 1.8e+02) false false))
        (:then_3
          (Transformation|SetRelativeRotation (Variables|Default|Get왼쪽30도) (Math|Rotator|MakeRotator 0.0 _왼쪽30도 1.8e+02) false false))))))

(event EventBeginPlay)

(event Collision|EventActorBeginOverlap
  (params (OtherActor :type Actor%20Object%20Reference)))

(event EventTick
  (params (DeltaSeconds :type Float%20%28single-precision%29)))

(fn ConstructionScript)