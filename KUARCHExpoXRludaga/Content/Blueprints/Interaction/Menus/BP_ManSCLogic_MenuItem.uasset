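; Menu item actor that shows one row of an interactive menu and reports its activation to the owning table.
; ChangeRow stores the row and unhides the item, and Tick refreshes its title and optional variable text while available.
; Tick also polls Activated, using paired DoOnce nodes to gate the ButtonClickMessage sent to TableOwner.
; HideButton toggles visibility of the text and target components and disables that Tick logic.
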(event Custom|ChangeRow
  (params (New%20Row :type Menu%20Row%20Struct%20Structure))
  (Variables|Default|SetMenuRow New%20Row)
  (CallFunction|HideButton false))

(event EventBeginPlay
  (|CallParentFunction) ; This node is disabled and will not be called.\nDrag off pins to build functionality.
)

(event Collision|EventActorBeginOverlap
  (params (OtherActor :type Actor%20Object%20Reference)))

(event EventTick
  (params (DeltaSeconds :type Float%20%28single-precision%29))
  (bind _menurow (Variables|Default|GetMenuRow))
  (bind _vartext (Variables|Default|GetVarText))
  (bind (_uniquename _titletext _longtext _vartext_2) (Utilities|Struct|BreakMenuRow_Struct _menurow))
  (|CallParentFunction DeltaSeconds)
  (if (not (Variables|Default|GetNotAvailable))
    (Utilities|FlowControl|Sequence
      (:then_0
        (Rendering|Components|TextRender|SetText (Variables|Default|GetMenuText) _titletext)
        (Utilities|IsValid _vartext
          (:Is%20Valid
            (Rendering|Components|TextRender|SetText _vartext _vartext_2))))
      (:then_1
        (if (Variables|Default|GetActivated?)
          (Utilities|FlowControl|DoOnce false :!label _label
            (:Completed
              (Utilities|FlowControl|Sequence
                (:then_0
                  (Class|MenuInterface|ButtonClick(Message) (Variables|Default|GetTableOwner) (Variables|Default|GetMenuRow)))
                (:then_1
                  (goto _label_2 Reset)))))
          (else
            (Utilities|FlowControl|DoOnce false :!label _label_2
              (:Completed
                (Utilities|FlowControl|Sequence
                  (:then_1
                    (goto _label Reset)))))))))))

(fn ConstructionScript
  (|CallParentFunction))

(fn HideButton
  (params (NewHidden :type Boolean))
  (bind _vartext (Variables|Default|GetVarText))
  (Development|SetHiddeninGame (Variables|Default|GetMenuText) NewHidden false)
  (Variables|Default|SetNotAvailable NewHidden)
  (Utilities|IsValid _vartext
    (:Is%20Valid
      (Development|SetHiddeninGame _vartext NewHidden false))))