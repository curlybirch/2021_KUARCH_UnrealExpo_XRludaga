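; Prototype in-world menu display that pages through a table of menu rows on five physical push buttons, with exit, back and scroll controls.
; On BeginPlay it attaches logic actors to the buttons, then loads title and table from TableOwner, falling back to itself.
; LastIndex drives row refresh, page text and arrow visibility, while Back restores the previous table.
; Exit destroys the menu and its button actors; item click actions are unimplemented.
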(event Custom|OnUpdate
  (if (not (Variables|Default|GetDying))
    (CallFunction|UpdatePageText)
    (CallFunction|HideLeft)
    (CallFunction|HideRight)))

(event EventBeginPlay
  (|CallParentFunction)
  (Utilities|FlowControl|Sequence
    (:then_0
      ;[1 1 1] Initialize the physical buttons with logic
      (Utilities|FlowControl|Sequence
        (:then_0
          (CallFunction|SetInternalButtons))
        (:then_1
          (CallFunction|SetMenuItemButtons))))
    (:then_1
      ;[1 1 1] If No Table Owner Set, Check for Self-Host Table
      (Utilities|IsValid (Variables|Default|GetTableOwner)
        (:Is%20Valid
          _)
        (:Is%20Not%20Valid
          (Variables|Default|SetTableOwner self)))
      ;[1 1 1] Request Table and Title
      (bind (_menutable _title) (Class|MenuInterface|GetTable(Message) (Variables|Default|GetTableOwner)))
      (Rendering|Components|TextRender|SetText (Variables|Default|GetTitleText) _title)
      ;[1 1 1] Load New Table
      (CallFunction|ChangeTable _menutable)
      ;[1 1 1] Table Rows to Buttons
      (CallFunction|RefreshPage (Variables|Default|GetCurrentTable) (Variables|Default|GetLastIndex)))
    (:then_2
      (CallFunction|OnUpdate))))

(event Collision|EventActorBeginOverlap
  (params (OtherActor :type Actor%20Object%20Reference)))

(event EventTick
  (params (DeltaSeconds :type Float%20%28single-precision%29))
  (|CallParentFunction DeltaSeconds)
  (Utilities|FlowControl|Sequence))

(event EventButtonClick
  (params (Button :type Menu%20Row%20Struct%20Structure))
  (bind _uniquename (Utilities|Struct|BreakMenuRow_Struct Button))
  ;[1 1 1] Actions on Click
  (Utilities|FlowControl|Sequence
    (:then_0
      (if (.ReturnValue (Utilities|Map|Find (Variables|Default|GetInternalButtonTable) _uniquename))
        (CallFunction|InternalButtonActions _uniquename)
        (elif (.ReturnValue (Utilities|Map|Find (Variables|Default|GetTestMenuTable) _uniquename))
          (CallFunction|MenuItemActions _uniquename))))
    (:then_1
      (CallFunction|OnUpdate))))

(fn ConstructionScript
  (|CallParentFunction))

(fn SetInternalButtons
  (bind _internalbuttontable (Variables|Default|GetInternalButtonTable))
  (bind _exitscene (Variables|Default|GetExitScene))
  (bind _scrollrightscene (Variables|Default|GetScrollRightScene))
  (bind _rightbutton (Variables|Default|GetRightButton))
  (bind _righttext (Variables|Default|GetRightText))
  (bind _exitbutton (Variables|Default|GetExitButton))
  (bind _exittext (Variables|Default|GetExitText))
  (bind _backscene (Variables|Default|GetBackScene))
  (bind _backbutton (Variables|Default|GetBackButton))
  (bind _backtext (Variables|Default|GetBackText))
  (bind _scrollleftscene (Variables|Default|GetScrollLeftScene))
  (bind _leftbutton (Variables|Default|GetLeftButton))
  (bind _lefttext (Variables|Default|GetLeftText))
  ;[1 1 1] Internal Buttons
  (Utilities|FlowControl|Sequence
    (:then_0
      (bind _menulogic (CallFunction|AddLogictoMenuButton :MenuRow (.Value (Utilities|Map|Find _internalbuttontable "exit")) :Scene _exitscene :Mesh _exitbutton :MenuTextRender _exittext :TableOwner self :MovementConstraints (Utilities|Struct|MakeStruct_ConstraintContainer "NewEnumerator1" (Utilities|Struct|MakeStruct_ButtonConstraints false false -3.0 1.0 1.0 0.0 0.5) "(BoundsType_3_295CD98E4D2862A6B4052790986A46EA=NewEnumerator0,LockSpecifiedValue_5_1E8FC7F64E9F7D85E5F24A85E78A6CFA=0.000000,Min_7_2A1EBA064A0EA8126606B59CD598994E=0.000000,Max_9_CD75696C42CE808B0A8BE1B2E7D1E63E=0.000000,ResetOnDrop?_14_B5062806488C4B3CFA94728FF0322F7D=True)" "(BoundsType_3_295CD98E4D2862A6B4052790986A46EA=NewEnumerator0,LockSpecifiedValue_5_1E8FC7F64E9F7D85E5F24A85E78A6CFA=0.000000,Min_7_2A1EBA064A0EA8126606B59CD598994E=0.000000,Max_9_CD75696C42CE808B0A8BE1B2E7D1E63E=0.000000,ResetOnDrop?_14_B5062806488C4B3CFA94728FF0322F7D=True)" "(BoundsType_3_295CD98E4D2862A6B4052790986A46EA=NewEnumerator0,LockSpecifiedValue_5_1E8FC7F64E9F7D85E5F24A85E78A6CFA=0.000000,Min_7_2A1EBA064A0EA8126606B59CD598994E=0.000000,Max_9_CD75696C42CE808B0A8BE1B2E7D1E63E=0.000000,ResetOnDrop?_14_B5062806488C4B3CFA94728FF0322F7D=True)" "(BoundsType_3_295CD98E4D2862A6B4052790986A46EA=NewEnumerator0,LockSpecifiedValue_5_1E8FC7F64E9F7D85E5F24A85E78A6CFA=0.000000,Min_7_2A1EBA064A0EA8126606B59CD598994E=0.000000,Max_9_CD75696C42CE808B0A8BE1B2E7D1E63E=0.000000,HandAxisBinding_15_7791594F48674BE9C9DB8A83B34E0C75=NewEnumerator1,ResetOnDrop?_17_54497A634287FD69CB6B0ABA09C6D891=True)" "(BoundsType_3_295CD98E4D2862A6B4052790986A46EA=NewEnumerator0,LockSpecifiedValue_5_1E8FC7F64E9F7D85E5F24A85E78A6CFA=0.000000,Min_7_2A1EBA064A0EA8126606B59CD598994E=0.000000,Max_9_CD75696C42CE808B0A8BE1B2E7D1E63E=0.000000,HandAxisBinding_15_7791594F48674BE9C9DB8A83B34E0C75=NewEnumerator0,ResetOnDrop?_17_54497A634287FD69CB6B0ABA09C6D891=True)" "(BoundsType_3_295CD98E4D2862A6B4052790986A46EA=NewEnumerator0,LockSpecifiedValue_5_1E8FC7F64E9F7D85E5F24A85E78A6CFA=0.000000,Min_7_2A1EBA064A0EA8126606B59CD598994E=0.000000,Max_9_CD75696C42CE808B0A8BE1B2E7D1E63E=0.000000,HandAxisBinding_15_7791594F48674BE9C9DB8A83B34E0C75=NewEnumerator2,ResetOnDrop?_17_54497A634287FD69CB6B0ABA09C6D891=True)") :Options (Utilities|Struct|MakeStruct_SubOptions false true) :Tags (Utilities|Array|MakeArray "None")))
      (Utilities|Map|Add (Variables|Default|GetInternalButtonLogicMap) (Utilities|Name|MakeLiteralName "exit") (Utilities|Struct|MakeButtonComponentStruct _exitscene _exitbutton _exittext _menulogic)))
    (:then_1
      (bind _menulogic_2 (CallFunction|AddLogictoMenuButton :MenuRow (.Value (Utilities|Map|Find _internalbuttontable "back")) :Scene _backscene :Mesh _backbutton :MenuTextRender _backtext :TableOwner self :MovementConstraints (Utilities|Struct|MakeStruct_ConstraintContainer "NewEnumerator1" (Utilities|Struct|MakeStruct_ButtonConstraints false false -3.0 1.0 1.0 0.0 0.5) "(BoundsType_3_295CD98E4D2862A6B4052790986A46EA=NewEnumerator0,LockSpecifiedValue_5_1E8FC7F64E9F7D85E5F24A85E78A6CFA=0.000000,Min_7_2A1EBA064A0EA8126606B59CD598994E=0.000000,Max_9_CD75696C42CE808B0A8BE1B2E7D1E63E=0.000000,ResetOnDrop?_14_B5062806488C4B3CFA94728FF0322F7D=True)" "(BoundsType_3_295CD98E4D2862A6B4052790986A46EA=NewEnumerator0,LockSpecifiedValue_5_1E8FC7F64E9F7D85E5F24A85E78A6CFA=0.000000,Min_7_2A1EBA064A0EA8126606B59CD598994E=0.000000,Max_9_CD75696C42CE808B0A8BE1B2E7D1E63E=0.000000,ResetOnDrop?_14_B5062806488C4B3CFA94728FF0322F7D=True)" "(BoundsType_3_295CD98E4D2862A6B4052790986A46EA=NewEnumerator0,LockSpecifiedValue_5_1E8FC7F64E9F7D85E5F24A85E78A6CFA=0.000000,Min_7_2A1EBA064A0EA8126606B59CD598994E=0.000000,Max_9_CD75696C42CE808B0A8BE1B2E7D1E63E=0.000000,ResetOnDrop?_14_B5062806488C4B3CFA94728FF0322F7D=True)" "(BoundsType_3_295CD98E4D2862A6B4052790986A46EA=NewEnumerator0,LockSpecifiedValue_5_1E8FC7F64E9F7D85E5F24A85E78A6CFA=0.000000,Min_7_2A1EBA064A0EA8126606B59CD598994E=0.000000,Max_9_CD75696C42CE808B0A8BE1B2E7D1E63E=0.000000,HandAxisBinding_15_7791594F48674BE9C9DB8A83B34E0C75=NewEnumerator1,ResetOnDrop?_17_54497A634287FD69CB6B0ABA09C6D891=True)" "(BoundsType_3_295CD98E4D2862A6B4052790986A46EA=NewEnumerator0,LockSpecifiedValue_5_1E8FC7F64E9F7D85E5F24A85E78A6CFA=0.000000,Min_7_2A1EBA064A0EA8126606B59CD598994E=0.000000,Max_9_CD75696C42CE808B0A8BE1B2E7D1E63E=0.000000,HandAxisBinding_15_7791594F48674BE9C9DB8A83B34E0C75=NewEnumerator0,ResetOnDrop?_17_54497A634287FD69CB6B0ABA09C6D891=True)" "(BoundsType_3_295CD98E4D2862A6B4052790986A46EA=NewEnumerator0,LockSpecifiedValue_5_1E8FC7F64E9F7D85E5F24A85E78A6CFA=0.000000,Min_7_2A1EBA064A0EA8126606B59CD598994E=0.000000,Max_9_CD75696C42CE808B0A8BE1B2E7D1E63E=0.000000,HandAxisBinding_15_7791594F48674BE9C9DB8A83B34E0C75=NewEnumerator2,ResetOnDrop?_17_54497A634287FD69CB6B0ABA09C6D891=True)") :Options (Utilities|Struct|MakeStruct_SubOptions false true) :Tags (Utilities|Array|MakeArray "None")))
      (Utilities|Map|Add (Variables|Default|GetInternalButtonLogicMap) (Utilities|Name|MakeLiteralName "back") (Utilities|Struct|MakeButtonComponentStruct _backscene _backbutton _backtext _menulogic_2)))
    (:then_2
      (bind _menulogic_3 (CallFunction|AddLogictoMenuButton :MenuRow (.Value (Utilities|Map|Find _internalbuttontable "left")) :Scene _scrollleftscene :Mesh _leftbutton :MenuTextRender _lefttext :TableOwner self :MovementConstraints (Utilities|Struct|MakeStruct_ConstraintContainer "NewEnumerator1" (Utilities|Struct|MakeStruct_ButtonConstraints false false -3.0 1.0 1.0 0.0 0.5) "(BoundsType_3_295CD98E4D2862A6B4052790986A46EA=NewEnumerator0,LockSpecifiedValue_5_1E8FC7F64E9F7D85E5F24A85E78A6CFA=0.000000,Min_7_2A1EBA064A0EA8126606B59CD598994E=0.000000,Max_9_CD75696C42CE808B0A8BE1B2E7D1E63E=0.000000,ResetOnDrop?_14_B5062806488C4B3CFA94728FF0322F7D=True)" "(BoundsType_3_295CD98E4D2862A6B4052790986A46EA=NewEnumerator0,LockSpecifiedValue_5_1E8FC7F64E9F7D85E5F24A85E78A6CFA=0.000000,Min_7_2A1EBA064A0EA8126606B59CD598994E=0.000000,Max_9_CD75696C42CE808B0A8BE1B2E7D1E63E=0.000000,ResetOnDrop?_14_B5062806488C4B3CFA94728FF0322F7D=True)" "(BoundsType_3_295CD98E4D2862A6B4052790986A46EA=NewEnumerator0,LockSpecifiedValue_5_1E8FC7F64E9F7D85E5F24A85E78A6CFA=0.000000,Min_7_2A1EBA064A0EA8126606B59CD598994E=0.000000,Max_9_CD75696C42CE808B0A8BE1B2E7D1E63E=0.000000,ResetOnDrop?_14_B5062806488C4B3CFA94728FF0322F7D=True)" "(BoundsType_3_295CD98E4D2862A6B4052790986A46EA=NewEnumerator0,LockSpecifiedValue_5_1E8FC7F64E9F7D85E5F24A85E78A6CFA=0.000000,Min_7_2A1EBA064A0EA8126606B59CD598994E=0.000000,Max_9_CD75696C42CE808B0A8BE1B2E7D1E63E=0.000000,HandAxisBinding_15_7791594F48674BE9C9DB8A83B34E0C75=NewEnumerator1,ResetOnDrop?_17_54497A634287FD69CB6B0ABA09C6D891=True)" "(BoundsType_3_295CD98E4D2862A6B4052790986A46EA=NewEnumerator0,LockSpecifiedValue_5_1E8FC7F64E9F7D85E5F24A85E78A6CFA=0.000000,Min_7_2A1EBA064A0EA8126606B59CD598994E=0.000000,Max_9_CD75696C42CE808B0A8BE1B2E7D1E63E=0.000000,HandAxisBinding_15_7791594F48674BE9C9DB8A83B34E0C75=NewEnumerator0,ResetOnDrop?_17_54497A634287FD69CB6B0ABA09C6D891=True)" "(BoundsType_3_295CD98E4D2862A6B4052790986A46EA=NewEnumerator0,LockSpecifiedValue_5_1E8FC7F64E9F7D85E5F24A85E78A6CFA=0.000000,Min_7_2A1EBA064A0EA8126606B59CD598994E=0.000000,Max_9_CD75696C42CE808B0A8BE1B2E7D1E63E=0.000000,HandAxisBinding_15_7791594F48674BE9C9DB8A83B34E0C75=NewEnumerator2,ResetOnDrop?_17_54497A634287FD69CB6B0ABA09C6D891=True)") :Options (Utilities|Struct|MakeStruct_SubOptions false true) :Tags (Utilities|Array|MakeArray "None")))
      (Utilities|Map|Add (Variables|Default|GetInternalButtonLogicMap) (Utilities|Name|MakeLiteralName "left") (Utilities|Struct|MakeButtonComponentStruct _scrollleftscene _leftbutton _lefttext _menulogic_3)))
    (:then_3
      (bind _menulogic_4 (CallFunction|AddLogictoMenuButton :MenuRow (.Value (Utilities|Map|Find _internalbuttontable "right")) :Scene _scrollrightscene :Mesh _rightbutton :MenuTextRender _righttext :TableOwner self :MovementConstraints (Utilities|Struct|MakeStruct_ConstraintContainer "NewEnumerator1" (Utilities|Struct|MakeStruct_ButtonConstraints false false -3.0 1.0 1.0 0.0 0.5) "(BoundsType_3_295CD98E4D2862A6B4052790986A46EA=NewEnumerator0,LockSpecifiedValue_5_1E8FC7F64E9F7D85E5F24A85E78A6CFA=0.000000,Min_7_2A1EBA064A0EA8126606B59CD598994E=0.000000,Max_9_CD75696C42CE808B0A8BE1B2E7D1E63E=0.000000,ResetOnDrop?_14_B5062806488C4B3CFA94728FF0322F7D=True)" "(BoundsType_3_295CD98E4D2862A6B4052790986A46EA=NewEnumerator0,LockSpecifiedValue_5_1E8FC7F64E9F7D85E5F24A85E78A6CFA=0.000000,Min_7_2A1EBA064A0EA8126606B59CD598994E=0.000000,Max_9_CD75696C42CE808B0A8BE1B2E7D1E63E=0.000000,ResetOnDrop?_14_B5062806488C4B3CFA94728FF0322F7D=True)" "(BoundsType_3_295CD98E4D2862A6B4052790986A46EA=NewEnumerator0,LockSpecifiedValue_5_1E8FC7F64E9F7D85E5F24A85E78A6CFA=0.000000,Min_7_2A1EBA064A0EA8126606B59CD598994E=0.000000,Max_9_CD75696C42CE808B0A8BE1B2E7D1E63E=0.000000,ResetOnDrop?_14_B5062806488C4B3CFA94728FF0322F7D=True)" "(BoundsType_3_295CD98E4D2862A6B4052790986A46EA=NewEnumerator0,LockSpecifiedValue_5_1E8FC7F64E9F7D85E5F24A85E78A6CFA=0.000000,Min_7_2A1EBA064A0EA8126606B59CD598994E=0.000000,Max_9_CD75696C42CE808B0A8BE1B2E7D1E63E=0.000000,HandAxisBinding_15_7791594F48674BE9C9DB8A83B34E0C75=NewEnumerator1,ResetOnDrop?_17_54497A634287FD69CB6B0ABA09C6D891=True)" "(BoundsType_3_295CD98E4D2862A6B4052790986A46EA=NewEnumerator0,LockSpecifiedValue_5_1E8FC7F64E9F7D85E5F24A85E78A6CFA=0.000000,Min_7_2A1EBA064A0EA8126606B59CD598994E=0.000000,Max_9_CD75696C42CE808B0A8BE1B2E7D1E63E=0.000000,HandAxisBinding_15_7791594F48674BE9C9DB8A83B34E0C75=NewEnumerator0,ResetOnDrop?_17_54497A634287FD69CB6B0ABA09C6D891=True)" "(BoundsType_3_295CD98E4D2862A6B4052790986A46EA=NewEnumerator0,LockSpecifiedValue_5_1E8FC7F64E9F7D85E5F24A85E78A6CFA=0.000000,Min_7_2A1EBA064A0EA8126606B59CD598994E=0.000000,Max_9_CD75696C42CE808B0A8BE1B2E7D1E63E=0.000000,HandAxisBinding_15_7791594F48674BE9C9DB8A83B34E0C75=NewEnumerator2,ResetOnDrop?_17_54497A634287FD69CB6B0ABA09C6D891=True)") :Options (Utilities|Struct|MakeStruct_SubOptions false true) :Tags (Utilities|Array|MakeArray "None")))
      (Utilities|Map|Add (Variables|Default|GetInternalButtonLogicMap) (Utilities|Name|MakeLiteralName "right") (Utilities|Struct|MakeButtonComponentStruct _scrollrightscene _rightbutton _righttext _menulogic_4)))))

(fn SetMenuItemButtons
  (bind _item0text (Variables|Default|GetItem0Text))
  (bind _item1scene (Variables|Default|GetItem1Scene))
  (bind _item1button (Variables|Default|GetItem1Button))
  (bind _item1vartext (Variables|Default|GetItem1VarText))
  (bind _item1text (Variables|Default|GetItem1Text))
  (bind _item2scene (Variables|Default|GetItem2Scene))
  (bind _item2button (Variables|Default|GetItem2Button))
  (bind _item2vartext (Variables|Default|GetItem2VarText))
  (bind _item2text (Variables|Default|GetItem2Text))
  (bind _item3scene (Variables|Default|GetItem3Scene))
  (bind _item3button (Variables|Default|GetItem3Button))
  (bind _item3vartext (Variables|Default|GetItem3VarText))
  (bind _item3text (Variables|Default|GetItem3Text))
  (bind _item4scene (Variables|Default|GetItem4Scene))
  (bind _item4button (Variables|Default|GetItem4Button))
  (bind _item4vartext (Variables|Default|GetItem4VarText))
  (bind _item4text (Variables|Default|GetItem4Text))
  (bind _item0scene (Variables|Default|GetItem0Scene))
  (bind _item0button (Variables|Default|GetItem0Button))
  (bind _item0vartext (Variables|Default|GetItem0VarText))
  (Utilities|FlowControl|Sequence
    (:then_0
      (bind _menulogic (CallFunction|AddLogictoMenuButton :MenuRow (Utilities|Struct|MakeMenuRow_Struct "0" "0" "0" "0") :Scene _item0scene :Mesh _item0button :MenuTextRender _item0text :VarText _item0vartext :MovementConstraints (Variables|Default|GetDefaultButtonSettings) :Options (Utilities|Struct|MakeStruct_SubOptions false true) :Tags (Utilities|Array|MakeArray "None")))
      (Utilities|Map|Add (Variables|Default|GetMenuItemButtonsLogicMap) 0 (Utilities|Struct|MakeButtonComponentStruct _item0scene _item0button _item0text _menulogic _item0vartext)))
    (:then_1
      (bind _menulogic_2 (CallFunction|AddLogictoMenuButton :MenuRow (Utilities|Struct|MakeMenuRow_Struct "1" "1" "1" "1") :Scene _item1scene :Mesh _item1button :MenuTextRender _item1text :VarText _item1vartext :MovementConstraints (Variables|Default|GetDefaultButtonSettings) :Options (Utilities|Struct|MakeStruct_SubOptions false true) :Tags (Utilities|Array|MakeArray "None")))
      (Utilities|Map|Add (Variables|Default|GetMenuItemButtonsLogicMap) 1 (Utilities|Struct|MakeButtonComponentStruct _item1scene _item1button _item1text _menulogic_2 _item1vartext)))
    (:then_2
      (bind _menulogic_3 (CallFunction|AddLogictoMenuButton :MenuRow (Utilities|Struct|MakeMenuRow_Struct "2" "2" "2" "2") :Scene _item2scene :Mesh _item2button :MenuTextRender _item2text :VarText _item2vartext :MovementConstraints (Variables|Default|GetDefaultButtonSettings) :Options (Utilities|Struct|MakeStruct_SubOptions false true) :Tags (Utilities|Array|MakeArray "None")))
      (Utilities|Map|Add (Variables|Default|GetMenuItemButtonsLogicMap) 2 (Utilities|Struct|MakeButtonComponentStruct _item2scene _item2button _item2text _menulogic_3 _item2vartext)))
    (:then_3
      (bind _menulogic_4 (CallFunction|AddLogictoMenuButton :MenuRow (Utilities|Struct|MakeMenuRow_Struct "3" "3" "3" "3") :Scene _item3scene :Mesh _item3button :MenuTextRender _item3text :VarText _item3vartext :MovementConstraints (Variables|Default|GetDefaultButtonSettings) :Options (Utilities|Struct|MakeStruct_SubOptions false true) :Tags (Utilities|Array|MakeArray "None")))
      (Utilities|Map|Add (Variables|Default|GetMenuItemButtonsLogicMap) 3 (Utilities|Struct|MakeButtonComponentStruct _item3scene _item3button _item3text _menulogic_4 _item3vartext)))
    (:then_4
      (bind _menulogic_5 (CallFunction|AddLogictoMenuButton :MenuRow (Utilities|Struct|MakeMenuRow_Struct "4" "4" "4" "4") :Scene _item4scene :Mesh _item4button :MenuTextRender _item4text :VarText _item4vartext :MovementConstraints (Variables|Default|GetDefaultButtonSettings) :Options (Utilities|Struct|MakeStruct_SubOptions false true) :Tags (Utilities|Array|MakeArray "None")))
      (Utilities|Map|Add (Variables|Default|GetMenuItemButtonsLogicMap) 4 (Utilities|Struct|MakeButtonComponentStruct _item4scene _item4button _item4text _menulogic_5 _item4vartext)))))

(fn RefreshPage
  (params (TargetTable :type Map%20of%20Names%20to%20Structs) (TableIndex :type Integer))
  (bind _values (Utilities|Map|Values (Variables|Default|GetMenuItemButtonsLogicMap)))
  (bind _values_2 (Utilities|Map|Values TargetTable))
  (for (_array_element _array_index) _values
    (if (Utilities|Array|IsValidIndex _values_2 (+ TableIndex _array_index))
      (Variables|Default|SetLastIndex (Math|Integer|Min(Integer) (Utilities|Map|Length TargetTable) (+ (Variables|Default|GetLastIndex) 1)))
      (Default|ChangeRow (.LogicBP (Utilities|Struct|BreakButtonComponentStruct _array_element)) (Utilities|Array|Get(acopy) _values_2 (+ TableIndex _array_index)))
      (else
        (Default|HideButton (.LogicBP (Utilities|Struct|BreakButtonComponentStruct _array_element)) true)))))

(fn ChangeTable
  (params (NewTable :type Map%20of%20Names%20to%20Structs))
  (Variables|Default|SetPreviousTable (Variables|Default|GetCurrentTable))
  (Variables|Default|SetCurrentTable NewTable)
  (Variables|Default|SetLastIndex 0))

(fn KillMenu
  (Variables|Default|SetDying true)
  (bind _values (Utilities|Map|Values (Variables|Default|GetInternalButtonLogicMap)))
  (for _array_element _values
    (Actor|DestroyActor (.LogicBP (Utilities|Struct|BreakButtonComponentStruct _array_element))))
  (bind _values_2 (Utilities|Map|Values (Variables|Default|GetMenuItemButtonsLogicMap)))
  (for _array_element_2 _values_2
    (Actor|DestroyActor (.LogicBP (Utilities|Struct|BreakButtonComponentStruct _array_element_2))))
  (Actor|DestroyActor))

(fn HideLeft
  (bind _internalbuttonlogicmap (Variables|Default|GetInternalButtonLogicMap))
  (bind _value (Utilities|Map|Find _internalbuttonlogicmap "left"))
  (bind _logicbp (Utilities|Struct|BreakButtonComponentStruct _value))
  (if (<= (Variables|Default|GetLastIndex) (Utilities|Map|Length (Variables|Default|GetMenuItemButtonsLogicMap)))
    (Default|HideButton _logicbp true)
    (else
      (Default|HideButton _logicbp false))))

(fn HideRight
  (bind _internalbuttonlogicmap (Variables|Default|GetInternalButtonLogicMap))
  (bind _value (Utilities|Map|Find _internalbuttonlogicmap "right"))
  (bind _logicbp (Utilities|Struct|BreakButtonComponentStruct _value))
  (if (>= (Variables|Default|GetLastIndex) (Utilities|Map|Length (Variables|Default|GetCurrentTable)))
    (Default|HideButton _logicbp true)
    (else
      (Default|HideButton _logicbp false))))

(fn InternalButtonActions
  (params (Selection :type Name))
  (switch name Selection
    (:exit
      (CallFunction|KillMenu))
    (:back
      (CallFunction|ChangeTable (Variables|Default|GetPreviousTable))
      (CallFunction|RefreshPage (Variables|Default|GetCurrentTable) (Variables|Default|GetLastIndex)))
    (:left
      (Variables|Default|SetLastIndex (Math|Integer|Max(Integer) (- (Variables|Default|GetLastIndex) (* (Utilities|Map|Length (Variables|Default|GetMenuItemButtonsLogicMap)) 2))))
      (CallFunction|RefreshPage (Variables|Default|GetCurrentTable) (Variables|Default|GetLastIndex)))
    (:right
      (CallFunction|RefreshPage (Variables|Default|GetCurrentTable) (Variables|Default|GetLastIndex)))))

(fn MenuItemActions
  (params (Selection :type Name))
  (switch name Selection))

(fn UpdatePageText
  (bind _menuitembuttonslogicmap (Variables|Default|GetMenuItemButtonsLogicMap))
  (bind _returnvalue (Utilities|Map|Length _menuitembuttonslogicmap))
  (bind _returnvalue_2 (Math|Conversions|ToFloat(Integer) _returnvalue))
  (Rendering|Components|TextRender|SetText (Variables|Default|GetPageNumText) (Utilities|Text|ToText(String) (Utilities|String|Append (Utilities|String|ToString(Integer) (Math|Float|Ceil (/ (Math|Conversions|ToFloat(Integer) (Variables|Default|GetLastIndex)) _returnvalue_2))) " / " (Utilities|String|ToString(Integer) (Math|Float|Ceil (/ (Math|Conversions|ToFloat(Integer) (Utilities|Map|Length (Variables|Default|GetCurrentTable))) _returnvalue_2)))))))

(fn GetTable
  (return (Variables|Default|GetTestMenuTable) "Test Menu"))