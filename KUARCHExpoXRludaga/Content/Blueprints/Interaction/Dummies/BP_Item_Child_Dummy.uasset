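; Dummy child of a base interaction item, serving as a test template for manipulable items with subcomponents.
; CustomizeSubcomponents spawns a BP_ManSCLogic for one button subcomponent with movement constraints and registers it in SubComponentMap as a magwell-attachable anchor.
; Tick optionally searches for a hang target, then previews (empty stub) or drops.
; Test activation logic swaps the base material with auto-deactivation; helper macros cover subcomponent building, activity branching and resettable DoOnce, largely left unwired.
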(event EventBeginPlay
  ;[1 1 1] Start
  (|CallParentFunction))

(event EventTick
  (params (DeltaSeconds :type Float%20%28single-precision%29))
  ;[1 1 1] Tick
  (|CallParentFunction DeltaSeconds)
  (Utilities|FlowControl|Sequence
    (:then_1
      (if (Variables|Default|GetSearchHangConstant?)
        (CallFunction|SearchHangTarget)
        (Utilities|IsValid (Variables|Default|GetHangTarget)
          (:Is%20Valid
            (if (Variables|Default|GetHangDropOnly?)
              (CallFunction|HangPreview)
              (else
                (CallFunction|ItemDropped)))))))))

(event Custom|CheckActivation
  (Utilities|FlowControl|Sequence
    (:then_0
      ;[1 1 1] Activation state of the base item
      (if (Variables|Default|GetActivated?)
        ;[1 0.4875 0] Default Base Item Activation for Testing
        (CallFunction|ActivateBaseItem)
        (Utilities|AutoBaseDeactivate 0.1)
        (else
          (CallFunction|DeactivateBaseItem))))
    (:then_1
      ;[1 1 1] Manually Cycle through SubComponents
      (Utilities|FlowControl|Sequence
        (:then_0
          ;[1 0.4875 0] Default SubComponent Activation for Testing
          (Utilities|SubActivityBranch))
        (:then_1
          (Utilities|SubActivityBranch 1))))))

(fn ConstructionScript
  (|CallParentFunction))

(fn ActiveComponentActions
  (params (TargetComponent :type Scene%20Component%20Object%20Reference) (Activated? :type Boolean))
  (switch int 0))

(fn ActiveItemActions
  (params (Activated? :type Boolean))
  (|CallParentFunction false))

(fn ManipulatedComponentActions
  (params (Component%20Struct :type Struct%20Item%20Sub%20Comp%20Properties%20Structure%20%28by%20ref%29)))

(fn CustomizeSubcomponents
  (bind _man0scene (Variables|Default|GetMan0Scene))
  (bind _man0mesh (Variables|Default|GetMan0Mesh))
  (bind _man0highlighter (Variables|Default|GetMan0Highlighter))
  ;[1 1 1] SetupManComps
  (Utilities|FlowControl|Sequence
    (:then_0
      ;[1 1 1] All the Sub Component-specific variables and logic live here
      (bind _returnvalue (Game|SpawnActorfromClass "/Game/Blueprints/Interaction/BP_ManSCLogic.BP_ManSCLogic_C" (Transformation|GetActorTransform) "AlwaysSpawn" 0 self "0.000000,0.000000,0.000000" (Utilities|Array|MakeArray (Transformation|GetRelativeTransform _man0scene)) _man0mesh "0.000000,0.000000,0.000000" (Variables|Default|GetMan0HandGhost) false _man0scene true false (Utilities|Struct|MakeStruct_ConstraintContainer "NewEnumerator1" (Utilities|Struct|MakeStruct_ButtonConstraints false false -1e+01 1e+01 0.0 0.0 0.0 0.0 3e+01) (Utilities|Struct|MakeStruct_LinearConstraints "NewEnumerator0" 0.0) (Utilities|Struct|MakeStruct_LinearConstraints "NewEnumerator0" 0.0) (Utilities|Struct|MakeStruct_LinearConstraints "NewEnumerator0" 0.0 25.0 1e+02) (Utilities|Struct|MakeStruct_AngularConstraints "NewEnumerator0" 0.0) (Utilities|Struct|MakeStruct_AngularConstraints "NewEnumerator0" 0.0 0.0 0.0 "NewEnumerator0") (Utilities|Struct|MakeStruct_AngularConstraints "NewEnumerator0" 0.0 0.0 0.0 "NewEnumerator2") (Utilities|Struct|MakeStruct_RadialConstraints false "NewEnumerator2")) _man0highlighter "NewEnumerator1" 1.0 true false 0))
      ;[1 1 1] For Use by Item BP
      (Utilities|Map|Add (Variables|Default|GetSubComponentMap) _man0mesh (Utilities|Struct|MakeStruct_ItemSubCompProperties _man0mesh _man0scene _man0highlighter _returnvalue (Utilities|Struct|MakeMaleAttacherStruct true (Utilities|Array|MakeArray "magwell") (Variables|Default|GetAttach0Ref)) (Utilities|Struct|MakeFemaleAttacherStruct false "(\"\")" 0 false) false true)))))

(fn ActivateBaseItem
  (Rendering|Material|SetMaterial (Variables|Default|GetBaseMesh) 0 "/Engine/VREditor/BasicMeshes/MI_Cube_02.MI_Cube_02"))

(fn DeactivateBaseItem
  (Rendering|Material|SetMaterial (Variables|Default|GetBaseMesh) 0 "/Engine/VREditor/BasicMeshes/MI_Cube_01.MI_Cube_01"))

(fn HangPreview)