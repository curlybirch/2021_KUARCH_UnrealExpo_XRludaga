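; Prototype stay-put dummy item with a grabbable bob that swings on a cable from a base mesh.
; BeginPlay registers the bob as an anchored sub-component driven by a spawned BP_ManSCLogic.
; Each tick, hand-rolled pendulum physics switches between free fall when slack and damped tangential gravity when taut, using polar conversion to hold cable length.
; Bob velocity feeds the logic actor's ExtraVelocity, with arrows and text showing debug state.
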(event EventBeginPlay
  (bind _man0scene (Variables|Default|GetMan0Scene))
  (bind _man0mesh (Variables|Default|GetMan0Mesh))
  (bind _man0highlighter (Variables|Default|GetMan0Highlighter))
  (bind _primaryghosthand (Variables|Default|GetPrimaryGhostHand))
  (bind _returnvalue (Transformation|GetRelativeTransform _primaryghosthand))
  (|CallParentFunction)
  (Utilities|FlowControl|Sequence
    (:then_0
      ;[1 0.2679 0] Customize Item Here
      (Utilities|FlowControl|Sequence
        (:then_0
          ;[1 0.7633 0] Determine placement in hand when gripped
          (Variables|Default|SetHandOffset (Math|Transform|MakeTransform (.location _returnvalue) (.rotation _returnvalue) "1,1,1"))
          ;[1 1 1] The green and blue arrows both fall along this axis
          (Variables|Default|SetReflectionAxis (Utilities|Enum|LiteralenumAxisEnum "NewEnumerator0"))
          ;[1 1 1] Hand pose when gripped
          (Variables|Default|SetGripType "NewEnumerator3")
          (Variables|Default|SetGripOverride 0.8))
        (:then_1
          ;[1 0.7388 0] Item Dropped only on second grip start
          (Variables|Default|SetSticky? false)
          ;[1 0.75 0] Item cannot be picked up, only manipulated/activated
          (Variables|Default|SetStayPut? true)
          ;[1 0.75 0] Base Item is Inactive
          (Variables|Default|SetDummy? true)
          ;[1 0.8032 0] Look for hang targets on tick or only on drop?
          (Variables|Default|SetSearchHangConstant? false)
          ;[1 0.9595 0] Hang on valid targets only when dropped, or as soon as acquired?
          (Variables|Default|SetHangDropOnly? true))))
    (:then_1
      (Utilities|FlowControl|Sequence
        (:then_0
          ;[1 1 1] SetupManComps
          (Utilities|FlowControl|Sequence
            (:then_0
              ;[1 1 1] All the Sub Component-specific variables and logic live here
              (bind _returnvalue_2 (Game|SpawnActorfromClass "/Game/Blueprints/Interaction/BP_ManSCLogic.BP_ManSCLogic_C" (Transformation|GetActorTransform) "AlwaysSpawn" 0 self "0.000000,0.000000,0.000000" (Utilities|Array|MakeArray (Transformation|GetRelativeTransform _man0scene)) _man0mesh "0.000000,0.000000,0.000000" (Variables|Default|GetMan0HandGhost) true _man0scene true true (Utilities|Struct|MakeStruct_ConstraintContainer "NewEnumerator1" (Utilities|Struct|MakeStruct_ButtonConstraints false false -1e+01 1e+01) (Utilities|Struct|MakeStruct_LinearConstraints "NewEnumerator0" 0.0) (Utilities|Struct|MakeStruct_LinearConstraints "NewEnumerator0" 0.0) (Utilities|Struct|MakeStruct_LinearConstraints "NewEnumerator0" 0.0 25.0 1e+02) (Utilities|Struct|MakeStruct_AngularConstraints "NewEnumerator0" 0.0) (Utilities|Struct|MakeStruct_AngularConstraints "NewEnumerator0" 0.0 0.0 0.0 "NewEnumerator0") (Utilities|Struct|MakeStruct_AngularConstraints "NewEnumerator0" 0.0 0.0 0.0 "NewEnumerator2") (Utilities|Struct|MakeStruct_RadialConstraints false "NewEnumerator2")) _man0highlighter "NewEnumerator1" 1.0 false false 0))
              ;[1 1 1] For Use by Item BP
              (Utilities|Map|Add (Variables|Default|GetSubComponentMap) _man0mesh (Utilities|Struct|MakeStruct_ItemSubCompProperties _man0mesh _man0scene _man0highlighter _returnvalue_2 (Utilities|Struct|MakeMaleAttacherStruct false (Utilities|Array|MakeArray "None")) (Utilities|Struct|MakeFemaleAttacherStruct false (Utilities|Array|MakeArray "None") 0 false) false true))
              (Variables|Default|SetSwingLogic _returnvalue_2))))
        (:then_1
          (bind _values (Utilities|Map|Values (Variables|Default|GetSubComponentMap)))
          (Variables|Default|SetSubComponentArray _values))))))

(event Collision|EventActorBeginOverlap
  (params (OtherActor :type Actor%20Object%20Reference)))

(event EventTick
  (params (DeltaSeconds :type Float%20%28single-precision%29))
  (|CallParentFunction DeltaSeconds)
  (Utilities|FlowControl|Sequence
    (:then_0
      (CallFunction|CablePhysics))))

(event Custom|Cable%20Physics
  (bind _returnvalue (Utilities|Time|GetWorldDeltaSeconds))
  (bind _returnvalue_2 (Utilities|Time|GetWorldDeltaSeconds))
  (bind _velocity (Variables|Default|GetVelocity))
  (bind _basemesh (Variables|Default|GetBaseMesh))
  (bind _man0scene (Variables|Default|GetMan0Scene))
  (bind _eq (Variables|Default|GetEQ))
  (bind _basemesh_2 (Variables|Default|GetBaseMesh))
  (bind _cableend (Variables|Default|GetCableEnd))
  (bind _returnvalue_3 (Transformation|GetWorldLocation _man0scene))
  (bind _returnvalue_4 (Transformation|GetWorldLocation _eq))
  (bind _returnvalue_5 (Transformation|GetWorldLocation _basemesh_2))
  (bind _returnvalue_6 (Transformation|GetWorldLocation _cableend))
  (bind _returnvalue_7 (Transformation|GetWorldLocation _basemesh))
  (bind _returnvalue_8 (Math|Rotator|FindLookatRotation _returnvalue_3 _returnvalue_4))
  (bind _returnvalue_9 (Math|Rotator|FindLookatRotation _returnvalue_5 _returnvalue_6))
  (bind _pitch (Math|Rotator|BreakRotator _returnvalue_9))
  (Utilities|FlowControl|Sequence
    (:then_0
      (Utilities|FlowControl|Sequence
        (:then_0
          (Utilities|FlowControl|Sequence
            (:then_0
              ;[1 1 1] Update Cable End
              (Transformation|SetWorldLocation (Variables|Default|GetCableEnd) (Transformation|GetWorldLocation (Variables|Default|GetMan0Scene)) false false)
              ;[1 1 1] Set Equilibrium Point
              (Transformation|SetWorldLocation (Variables|Default|GetEQ) (- (Transformation|GetWorldLocation (Variables|Default|GetBaseMesh)) (Math|Vector|MakeVector 0.0 0.0 (* (Variables|Default|GetMaxExtension) 0.8))) false false)
              (Variables|Default|SetLastTheta (Variables|Default|GetAngleTheta))
              (Variables|Default|SetAngleTheta (* (- 9e+01 (Math|Float|Absolute(Float) _pitch)) -1.0))
              (Rendering|Components|TextRender|SetText (Variables|Default|GetTextRender) (Utilities|Text|ToText(Float) _pitch "HalfToEven"))
              (Transformation|SetWorldRotation _velocity (Math|Conversions|RotationFromXVector (Variables|Default|GetBobVelocity)) false false)
              (Variables|/Script/Engine.ArrowComponent|SetArrowSize _velocity (/ (Variables|Default|GetBobSpeed) 1e+01)))
            (:then_1
              (if (Variables|Default|GetFreeFallMode)
                (Development|SetHiddeninGame (Variables|Default|GetAccArrow) true false)
                (Development|SetHiddeninGame (Variables|Default|GetGravArrow) false false)
                (Transformation|SetWorldRotation (Variables|Default|GetGravArrow) "-90.000000,0.000000, 0" false false)
                (else
                  (Development|SetHiddeninGame (Variables|Default|GetAccArrow) false false)
                  (Development|SetHiddeninGame (Variables|Default|GetGravArrow) true false)
                  ;[1 1 1] Point Arrow and Man Mesh Toward EQ
                  (Transformation|SetWorldRotation (Variables|Default|GetAccArrow) (Math|Rotator|MakeRotator (.roll _returnvalue_8) (.pitch _returnvalue_8) (.yaw _returnvalue_8)) false false))))))
        (:then_1
          ;[1 1 1] Get Cable State, Extended or Limp
          (bind _output_get (Variables|Default|SetCableExtension (Math|Vector|Distance(Vector) (Transformation|GetWorldLocation (Variables|Default|GetCable)) (Transformation|GetWorldLocation (Variables|Default|GetCableEnd)))))
          (if (< _output_get (- (Variables|Default|GetMaxExtension) 1.0))
            (Variables|Default|SetFreeFallMode true)
            (goto _label Reset)
            (else
              (Variables|Default|SetFreeFallMode false)
              (Utilities|FlowControl|Sequence
                (:then_0
                  (Utilities|FlowControl|DoOnce false :!label _label
                    (:Completed
                      (Variables|Default|SetBobVelocity (* (Math|Vector|GetUnitDirection(Vector) (Transformation|GetWorldLocation (Variables|Default|GetMan0Scene)) (Transformation|GetWorldLocation (Variables|Default|GetEQ))) (* (Variables|Default|GetBobSpeed) (Math|Float|Absolute(Float) (Math|Trig|Sin(Degrees) (Variables|Default|GetAngleTheta))))))
                      (Variables|Default|SetMaxTheta (* (Variables|Default|GetAngleTheta) 1.0)))))
                (:then_1
                  (if (Math|Float|NearlyEqual(Float) (Variables|Default|GetAngleTheta) 0.0 5.0)
                    (Utilities|FlowControl|DoOnce false
                      (:Completed
                        (goto _label_2 Open)))))))))
        (:then_2
          (if (Variables|Default|GetFreeFallMode)
            (Utilities|FlowControl|Sequence
              (:then_0
                ;[1 1 1] Pull Straight Down
                (bind _acceleration_vector (CallFunction|1DGrav -9.0 _returnvalue_2))
                (bind _output_get_2 (Variables|Default|SetBobVelocity (+ _acceleration_vector (Variables|Default|GetBobVelocity))))
                (Variables|Default|SetBobSpeed (Math|Vector|VectorLength _output_get_2))
                (Transformation|AddWorldOffset (Variables|Default|GetMan0Scene) (* _output_get_2 _returnvalue_2) false false)))
            (else
              (Utilities|FlowControl|Sequence
                (:then_0
                  (Variables|Default|SetSmallTheta (Math|Float|Min(Float) (Math|Float|Absolute(Float) (Variables|Default|GetMaxTheta)) (Math|Float|Absolute(Float) (Variables|Default|GetAngleTheta))))
                  ;[1 1 1] Acceleration Magnitude from Grav * sinTheta
                  (bind _acceleration_vector_2 (CallFunction|1DGrav -9.0 (Utilities|Time|GetWorldDeltaSeconds)))
                  (bind _output_get_3 (Variables|Default|SetBobVelocity (+ (* (Math|Vector|GetForwardVector (Variables|Default|GetAccArrow)) (* (Math|Vector|VectorLength _acceleration_vector_2) (Math|Float|Absolute(Float) (Math|Trig|Sin(Degrees) (Variables|Default|GetSmallTheta))))) (Variables|Default|GetBobVelocity))))
                  (Variables|Default|SetBobSpeed (Math|Vector|VectorLength _output_get_3))
                  (bind _polarrai (CallFunction|ConvertGridtoPolar (+ (* (Variables|Default|GetBobVelocity) (Utilities|Time|GetWorldDeltaSeconds)) (- (Transformation|GetWorldLocation (Variables|Default|GetMan0Scene)) _returnvalue_7))))
                  (bind _gridxyz (CallFunction|ConvertPolartoGrid (Utilities|Struct|MakeSphereCoordsStruct (Variables|Default|GetMaxExtension) (.azimuth _polarrai) (.inclination _polarrai))))
                  (Transformation|SetWorldLocation (Variables|Default|GetMan0Scene) (+ _gridxyz _returnvalue_7) false false)
                  (Utilities|FlowControl|Gate true :!label _label_2
                    (:Exit
                      (if (and (>= (Math|Float|Absolute(Float) (Variables|Default|GetAngleTheta)) (* (Math|Float|Absolute(Float) (Variables|Default|GetMaxTheta)) 0.5)) (> (Math|Float|Absolute(Float) (Variables|Default|GetAngleTheta)) (Math|Float|Absolute(Float) (Variables|Default|GetLastTheta))))
                        (Variables|Default|SetBobVelocity (- (Variables|Default|GetBobVelocity) (* (* (Variables|Default|GetBobVelocity) (* (+ (Math|Float|Absolute(Float) (Math|Trig|Sin(Degrees) (Variables|Default|GetAngleTheta))) 1.0) (Math|Float|Max(Float) (- (Math|Float|Absolute(Float) (Variables|Default|GetAngleTheta)) (Math|Float|Absolute(Float) (Variables|Default|GetMaxTheta))) 1.0) 1.0)) _returnvalue)))
                        (Variables|Default|SetMaxTheta (Math|Float|Min(Float) (+ (* _returnvalue (/ (Math|Float|Absolute(Float) (Variables|Default|GetMaxTheta)) 2.0) (Variables|Default|GetBrake)) (Variables|Default|GetMaxTheta)) 0.0))))))))))))
    (:then_1
      (Variables|/Game/Blueprints/Interaction/BP_ManSCLogic.BP_ManSCLogic_C|SetExtraVelocity (Variables|Default|GetSwingLogic) (Variables|Default|GetBobVelocity)))))

(fn ConstructionScript
  (|CallParentFunction))

(fn CustomizeBaseItem
  (|CallParentFunction))