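; Bogota interaction Blueprint that reveals three components, named for 0, 20 and 200 degrees (도), when their collision areas are overlapped.
; BeginPlay hides all three components.
; Each component has a matching collision component whose begin-overlap event unhides it, with no check on the overlapping actor.
; There is no end-overlap handling, so revealed components stay visible.
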(event OnComponentBeginOverlap(0도콜리전)
  (params (OverlappedComponent :type Primitive%20Component%20Object%20Reference) (OtherActor :type Actor%20Object%20Reference) (OtherComp :type Primitive%20Component%20Object%20Reference) (OtherBodyIndex :type Integer) (bFromSweep :type Boolean) (SweepResult :type Hit%20Result%20Structure%20%28by%20ref%29))
  (Development|SetHiddeninGame (Variables|Default|Get0도) false false))

(event OnComponentBeginOverlap(20도콜리전)
  (params (OverlappedComponent :type Primitive%20Component%20Object%20Reference) (OtherActor :type Actor%20Object%20Reference) (OtherComp :type Primitive%20Component%20Object%20Reference) (OtherBodyIndex :type Integer) (bFromSweep :type Boolean) (SweepResult :type Hit%20Result%20Structure%20%28by%20ref%29))
  (Development|SetHiddeninGame (Variables|Default|Get20도) false false))

(event OnComponentBeginOverlap(200도콜리전)
  (params (OverlappedComponent :type Primitive%20Component%20Object%20Reference) (OtherActor :type Actor%20Object%20Reference) (OtherComp :type Primitive%20Component%20Object%20Reference) (OtherBodyIndex :type Integer) (bFromSweep :type Boolean) (SweepResult :type Hit%20Result%20Structure%20%28by%20ref%29))
  (Development|SetHiddeninGame (Variables|Default|Get200도) false false))

(event EventBeginPlay
  (Utilities|FlowControl|Sequence
    (:then_0
      (Development|SetHiddeninGame (Variables|Default|Get0도) true false))
    (:then_1
      (Development|SetHiddeninGame (Variables|Default|Get20도) true false))
    (:then_2
      (Development|SetHiddeninGame (Variables|Default|Get200도) true false))))

(fn ConstructionScript)