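; Prototype VR pistol pickup, a child item that fires repeatedly while activated, using line traces with explosion impacts and brief muzzle sparks.
; BeginPlay registers sub-components for a constrained sliding handle, a grabbable foregrip and a socket accepting "mag"-tagged attachments.
; While the foregrip is held, Tick aims the gun using both hands.
; On foregrip release, a DoOnce detaches and re-picks it up with the owning hand.
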(event EventBeginPlay
  (bind _attach1ref (Variables|Default|GetAttach1Ref))
  (bind _handlescene1 (Variables|Default|GetHandleScene1))
  (|CallParentFunction)
  (Utilities|FlowControl|Sequence
    (:then_0
      (Variables|Default|SetHandOffset (Transformation|GetRelativeTransform (Variables|Default|GetPrimaryGhostHand)))
      (CallFunction|AddLogictoSubComponent (Variables|Default|GetHandleScene) (Variables|Default|GetMan0Mesh1) (Variables|Default|GetMan0Highlighter1) (Variables|Default|GetMan0HandGhost1) 0 0 (Utilities|Struct|MakeStruct_ConstraintContainer "NewEnumerator1" "(Toggleable?_3_35007B1949ABC9888873D4866C35477C=False,Sticky?_21_C890B630443EEB468DFF28843F253075=False,MinX_9_0FF88DFE4217FFF1EC905BB447CBF3B2=0.000000,MaxX_8_B370D57E443F5E0E24FDDABA0BA99C7D=0.000000,ResetX_11_5B812BFE4FD86D460FEE8198946B7B57=0.000000,ToggleX_13_DA5536974CA964836CF06BB91D709D40=0.000000,ActiveToggleOnThresh_15_E7080EA6454858B5DC8A948E40BC5BC1=0.000000,ToggleOffThresh_17_2D36698647CF2A7BF48E7FAB9BFEB092=0.000000,Speed_19_6497B3894B3DAA00D8E02C96A6FBEDC0=10.000000)" (Utilities|Struct|MakeStruct_LinearConstraints "NewEnumerator3" 0.0 -1e+02 -25.0) "(BoundsType_3_295CD98E4D2862A6B4052790986A46EA=NewEnumerator0,LockSpecifiedValue_5_1E8FC7F64E9F7D85E5F24A85E78A6CFA=0.000000,Min_7_2A1EBA064A0EA8126606B59CD598994E=0.000000,Max_9_CD75696C42CE808B0A8BE1B2E7D1E63E=0.000000,ResetOnDrop?_14_B5062806488C4B3CFA94728FF0322F7D=True)" "(BoundsType_3_295CD98E4D2862A6B4052790986A46EA=NewEnumerator0,LockSpecifiedValue_5_1E8FC7F64E9F7D85E5F24A85E78A6CFA=0.000000,Min_7_2A1EBA064A0EA8126606B59CD598994E=0.000000,Max_9_CD75696C42CE808B0A8BE1B2E7D1E63E=0.000000,ResetOnDrop?_14_B5062806488C4B3CFA94728FF0322F7D=True)" "(BoundsType_3_295CD98E4D2862A6B4052790986A46EA=NewEnumerator0,LockSpecifiedValue_5_1E8FC7F64E9F7D85E5F24A85E78A6CFA=0.000000,Min_7_2A1EBA064A0EA8126606B59CD598994E=0.000000,Max_9_CD75696C42CE808B0A8BE1B2E7D1E63E=0.000000,HandAxisBinding_15_7791594F48674BE9C9DB8A83B34E0C75=NewEnumerator1,ResetOnDrop?_17_54497A634287FD69CB6B0ABA09C6D891=True)" "(BoundsType_3_295CD98E4D2862A6B4052790986A46EA=NewEnumerator0,LockSpecifiedValue_5_1E8FC7F64E9F7D85E5F24A85E78A6CFA=0.000000,Min_7_2A1EBA064A0EA8126606B59CD598994E=0.000000,Max_9_CD75696C42CE808B0A8BE1B2E7D1E63E=0.000000,HandAxisBinding_15_7791594F48674BE9C9DB8A83B34E0C75=NewEnumerator0,ResetOnDrop?_17_54497A634287FD69CB6B0ABA09C6D891=True)" "(BoundsType_3_295CD98E4D2862A6B4052790986A46EA=NewEnumerator0,LockSpecifiedValue_5_1E8FC7F64E9F7D85E5F24A85E78A6CFA=0.000000,Min_7_2A1EBA064A0EA8126606B59CD598994E=0.000000,Max_9_CD75696C42CE808B0A8BE1B2E7D1E63E=0.000000,HandAxisBinding_15_7791594F48674BE9C9DB8A83B34E0C75=NewEnumerator2,ResetOnDrop?_17_54497A634287FD69CB6B0ABA09C6D891=True)") (Utilities|Struct|MakeStruct_GripOverrides "NewEnumerator1" 1.0) (Utilities|Struct|MakeStruct_SubOptions true false false false false true) (Utilities|Array|MakeArray "None"))
      (CallFunction|AddLogictoSubComponent :Scene (Variables|Default|GetForegripScene) :Mesh (Variables|Default|GetMan0Mesh2) :HighlightCap (Variables|Default|GetMan0Highlighter2) :Ghosthand (Variables|Default|GetPrimaryGhostHand1) :Grip (Utilities|Struct|MakeStruct_GripOverrides "NewEnumerator1" 1.0) :Options (Utilities|Struct|MakeStruct_SubOptions true false) :Tags (Utilities|Array|MakeArray "None"))
      (CallFunction|AddLogictoSubComponent :Scene _handlescene1 :Mesh (Variables|Default|GetMan0Mesh3) :HighlightCap (Variables|Default|GetMan0Highlighter3) :Ghosthand (Variables|Default|GetMan0HandGhost3) :FemaleAttScene _attach1ref :Options (Utilities|Struct|MakeStruct_SubOptions false false false false false false false (Utilities|Struct|MakeStruct_AttachContainer "(MaleAttachable?_11_368F68E44450541CCEBFB3B54FB02ED7=False,TagTargets_16_2D9CC1914C1287BD23D04C97999008CB=(\"\"),MaleAttachLocationRefScene_18_6280FEEA4917F131C383DFB5047871A9=None,OnDropOnly?_3_7FC864CD458A1BAB7B2D86AB7FB2D84C=True,Preview?_5_472DC8E24FE12446631A9E82B8367E64=False,AttachedNow?_7_8879E57F46776D842CB8A68460A1C8B4=False)" (Utilities|Struct|MakeFemaleAttacherStruct true (Utilities|Array|MakeArray "mag") _attach1ref false))) :Tags (Utilities|Array|MakeArray "None"))
      (Transformation|AttachComponentToComponent (Variables|Default|GetAttach1Ref) _handlescene1 "None" "KeepRelative" "KeepRelative" "KeepRelative" true))
    (:then_1
      ;[1 0.7388 0] Item Dropped only on second grip start
      (Variables|Default|SetSticky? false)
      ;[1 0.75 0] Item cannot be picked up, only manipulated/activated
      (Variables|Default|SetStayPut? false)
      ;[1 0.75 0] Base Item is Inactive
      (Variables|Default|SetDummy? false)
      ;[1 0.8032 0] Look for hang targets on tick or only on drop?
      (Variables|Default|SetSearchHangConstant? false)
      ;[1 0.9595 0] Hang on valid targets only when dropped, or as soon as acquired?
      (Variables|Default|SetHangDropOnly? true))))

(event Collision|EventActorBeginOverlap
  (params (OtherActor :type Actor%20Object%20Reference)))

(event EventTick
  (params (DeltaSeconds :type Float%20%28single-precision%29))
  (bind _man0scene (Variables|Default|GetMan0Scene))
  (bind _owninghand (Variables|Default|GetOwningHand))
  (bind _subcomponentmap (Variables|Default|GetSubComponentMap))
  (bind _man0mesh2 (Variables|Default|GetMan0Mesh2))
  (bind (_value _returnvalue) (Utilities|Map|Find _subcomponentmap _man0mesh2))
  (bind _returnvalue_2 (Transformation|GetWorldLocation _man0scene))
  (bind _asbp_vr_hand (Utilities|Casting|CastToBP_VR_Hand _owninghand))
  (bind _logicbp (Utilities|Struct|BreakStruct_ItemSubCompProperties _value))
  (bind _manipulatinghand (Variables|/Game/Blueprints/Interaction/BP_ManSCLogic.BP_ManSCLogic_C|GetManipulatingHand _logicbp))
  (bind _rootcomponent (Variables|/Script/Engine.Actor|GetRootComponent _manipulatinghand))
  (bind _returnvalue_3 (Transformation|GetWorldLocation _rootcomponent))
  (bind _returnvalue_4 (Math|Rotator|FindLookatRotation _returnvalue_3 _returnvalue_2))
  (|CallParentFunction DeltaSeconds)
  (Utilities|FlowControl|Sequence
    (:then_0
      (if (Variables|Default|GetActivated?)
        (Utilities|FlowControl|DoOnce false :!label _label
          (:Completed
            (Utilities|FlowControl|Sequence
              (:then_0
                (CallFunction|Shoot)
                (Utilities|BlastReport))
              (:then_1
                (Utilities|FlowControl|Delay 0.08)
                (goto _label Reset)))))))
    (:then_1
      (if _returnvalue
        (if (Variables|/Game/Blueprints/Interaction/BP_ManSCLogic.BP_ManSCLogic_C|GetManipulating _logicbp)
          (Transformation|SetActorRotation (Math|Rotator|MakeRotator (* (.roll (Transformation|GetWorldRotation (Variables|/Script/Engine.Actor|GetRootComponent _owninghand))) -1.0) (.pitch _returnvalue_4) (.yaw _returnvalue_4)))
          (goto _label_2 Reset)
          (elif (Variables|Default|GetHeld?)
            (Utilities|FlowControl|DoOnce true :!label _label_2
              (:Completed
                (Transformation|DetachFromActor "KeepWorld" "KeepWorld" "KeepWorld")
                (CallFunction|ItemPickedUp (Variables|/Game/Blueprints/Pawn/BP_VR_Hand.BP_VR_Hand_C|GetOwningPawn _asbp_vr_hand) _owninghand (Variables|/Game/Blueprints/Pawn/BP_VR_Hand.BP_VR_Hand_C|GetAttachScene _asbp_vr_hand))))))))))

(fn ConstructionScript
  (|CallParentFunction))

(fn Shoot
  (bind _attach0ref (Variables|Default|GetAttach0Ref))
  (bind _returnvalue (Transformation|GetWorldLocation _attach0ref))
  (bind (_outhit _returnvalue_2) (Collision|LineTraceByChannel _returnvalue (+ _returnvalue (* (Math|Vector|GetForwardVector _attach0ref) (Variables|Default|GetRange))) "TraceTypeQuery1" false 0 "ForOneFrame"))
  (if _returnvalue_2
    (bind _returnvalue_3 (Effects|SpawnEmitteratLocation "/Game/MobileStarterContent/Particles/P_Explosion.P_Explosion" (.ImpactPoint (Collision|BreakHitResult _outhit))))
    (Variables|/Script/Engine.ParticleSystemComponent|SetCustomTimeDilation _returnvalue_3 3.0)))