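; Prototype hand-grippable pickup item that sets up a manipulable, attachable sub-component on top of its parent pickup class.
; BeginPlay sets grip pose, hand offset from a ghost hand and drop/hang flags, then spawns a BP_ManSCLogic actor to drive Man0Mesh.
; It registers that mesh in SubComponentMap as both male attacher (targeting "magwell") and female attacher (accepting "fem"), then caches SubComponentArray.
; Unconnected leftover setup nodes never run.
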(event EventBeginPlay
  (bind _primaryghosthand (Variables|Default|GetPrimaryGhostHand))
  (bind _man0scene (Variables|Default|GetMan0Scene))
  (bind _man0highlighter (Variables|Default|GetMan0Highlighter))
  (bind _man0mesh (Variables|Default|GetMan0Mesh))
  (bind _returnvalue (Transformation|GetRelativeTransform _primaryghosthand))
  (|CallParentFunction)
  (Utilities|FlowControl|Sequence
    (:then_0
      ;[1 0.2679 0] Customize Item Here
      (Utilities|FlowControl|Sequence
        (:then_0
          ;[1 0.7633 0] Determine placement in hand when gripped
          (Variables|Default|SetHandOffset (Math|Transform|MakeTransform (.location _returnvalue) (.rotation _returnvalue) "1,1,1"))
          ;[1 1 1] The green and blue arrows both fall along this axis
          (Variables|Default|SetReflectionAxis (Utilities|Enum|LiteralenumAxisEnum "NewEnumerator0"))
          ;[1 1 1] Hand pose when gripped
          (Variables|Default|SetGripType "NewEnumerator3")
          (Variables|Default|SetGripOverride 0.8))
        (:then_1
          ;[1 0.7388 0] Item Dropped only on second grip start
          (Variables|Default|SetSticky? false)
          ;[1 0.75 0] Item cannot be picked up, only manipulated/activated
          (Variables|Default|SetStayPut? false)
          ;[1 0.75 0] Base Item is Inactive
          (Variables|Default|SetDummy? false)
          ;[1 0.8032 0] Look for hang targets on tick or only on drop?
          (Variables|Default|SetSearchHangConstant? false)
          ;[1 0.9595 0] Hang on valid targets only when dropped, or as soon as acquired?
          (Variables|Default|SetHangDropOnly? true))))
    (:then_1
      (Utilities|FlowControl|Sequence
        (:then_0
          ;[1 1 1] SetupManComps
          (Utilities|FlowControl|Sequence
            (:then_0
              ;[1 1 1] All the Sub Component-specific variables and logic live here
              (bind _returnvalue_2 (Game|SpawnActorfromClass "/Game/Blueprints/Interaction/BP_ManSCLogic.BP_ManSCLogic_C" (Transformation|GetActorTransform) "AlwaysSpawn" 0 self "0.000000,0.000000,0.000000" (Utilities|Array|MakeArray (Transformation|GetRelativeTransform _man0scene)) _man0mesh "0.000000,0.000000,0.000000" (Variables|Default|GetMan0HandGhost) false _man0scene false true (Utilities|Struct|MakeStruct_ConstraintContainer "NewEnumerator1" "(Toggleable?_3_35007B1949ABC9888873D4866C35477C=False,Sticky?_21_C890B630443EEB468DFF28843F253075=False,MinX_9_0FF88DFE4217FFF1EC905BB447CBF3B2=0.000000,MaxX_8_B370D57E443F5E0E24FDDABA0BA99C7D=0.000000,ResetX_11_5B812BFE4FD86D460FEE8198946B7B57=0.000000,ToggleX_13_DA5536974CA964836CF06BB91D709D40=0.000000,ActiveToggleOnThresh_15_E7080EA6454858B5DC8A948E40BC5BC1=0.000000,ToggleOffThresh_17_2D36698647CF2A7BF48E7FAB9BFEB092=0.000000,Speed_19_6497B3894B3DAA00D8E02C96A6FBEDC0=10.000000)" "(BoundsType_3_295CD98E4D2862A6B4052790986A46EA=NewEnumerator0,LockSpecifiedValue_5_1E8FC7F64E9F7D85E5F24A85E78A6CFA=0.000000,Min_7_2A1EBA064A0EA8126606B59CD598994E=0.000000,Max_9_CD75696C42CE808B0A8BE1B2E7D1E63E=0.000000,ResetOnDrop?_14_B5062806488C4B3CFA94728FF0322F7D=True)" "(BoundsType_3_295CD98E4D2862A6B4052790986A46EA=NewEnumerator0,LockSpecifiedValue_5_1E8FC7F64E9F7D85E5F24A85E78A6CFA=0.000000,Min_7_2A1EBA064A0EA8126606B59CD598994E=0.000000,Max_9_CD75696C42CE808B0A8BE1B2E7D1E63E=0.000000,ResetOnDrop?_14_B5062806488C4B3CFA94728FF0322F7D=True)" "(BoundsType_3_295CD98E4D2862A6B4052790986A46EA=NewEnumerator0,LockSpecifiedValue_5_1E8FC7F64E9F7D85E5F24A85E78A6CFA=0.000000,Min_7_2A1EBA064A0EA8126606B59CD598994E=0.000000,Max_9_CD75696C42CE808B0A8BE1B2E7D1E63E=0.000000,ResetOnDrop?_14_B5062806488C4B3CFA94728FF0322F7D=True)" "(BoundsType_3_295CD98E4D2862A6B4052790986A46EA=NewEnumerator0,LockSpecifiedValue_5_1E8FC7F64E9F7D85E5F24A85E78A6CFA=0.000000,Min_7_2A1EBA064A0EA8126606B59CD598994E=0.000000,Max_9_CD75696C42CE808B0A8BE1B2E7D1E63E=0.000000,HandAxisBinding_15_7791594F48674BE9C9DB8A83B34E0C75=NewEnumerator1,ResetOnDrop?_17_54497A634287FD69CB6B0ABA09C6D891=True)" "(BoundsType_3_295CD98E4D2862A6B4052790986A46EA=NewEnumerator0,LockSpecifiedValue_5_1E8FC7F64E9F7D85E5F24A85E78A6CFA=0.000000,Min_7_2A1EBA064A0EA8126606B59CD598994E=0.000000,Max_9_CD75696C42CE808B0A8BE1B2E7D1E63E=0.000000,HandAxisBinding_15_7791594F48674BE9C9DB8A83B34E0C75=NewEnumerator0,ResetOnDrop?_17_54497A634287FD69CB6B0ABA09C6D891=True)" "(BoundsType_3_295CD98E4D2862A6B4052790986A46EA=NewEnumerator0,LockSpecifiedValue_5_1E8FC7F64E9F7D85E5F24A85E78A6CFA=0.000000,Min_7_2A1EBA064A0EA8126606B59CD598994E=0.000000,Max_9_CD75696C42CE808B0A8BE1B2E7D1E63E=0.000000,HandAxisBinding_15_7791594F48674BE9C9DB8A83B34E0C75=NewEnumerator2,ResetOnDrop?_17_54497A634287FD69CB6B0ABA09C6D891=True)" (Utilities|Struct|MakeStruct_RadialConstraints false "NewEnumerator2")) _man0highlighter "NewEnumerator1" 1.0 false false 0))
              ;[1 1 1] For Use by Item BP
              (Utilities|Map|Add (Variables|Default|GetSubComponentMap) _man0mesh (Utilities|Struct|MakeStruct_ItemSubCompProperties _man0mesh _man0scene _man0highlighter _returnvalue_2 (Utilities|Struct|MakeMaleAttacherStruct true (Utilities|Array|MakeArray "magwell") (Variables|Default|GetAttach0Ref)) (Utilities|Struct|MakeFemaleAttacherStruct true (Utilities|Array|MakeArray "fem") (Variables|Default|GetAttach1Ref) false))))))
        (:then_1
          (bind _values (Utilities|Map|Values (Variables|Default|GetSubComponentMap)))
          (Variables|Default|SetSubComponentArray _values))))))

(event Collision|EventActorBeginOverlap
  (params (OtherActor :type Actor%20Object%20Reference)))

(event EventTick
  (params (DeltaSeconds :type Float%20%28single-precision%29))
  (|CallParentFunction DeltaSeconds) ; This node is disabled and will not be called.\nDrag off pins to build functionality.
)

(fn ConstructionScript
  (|CallParentFunction))