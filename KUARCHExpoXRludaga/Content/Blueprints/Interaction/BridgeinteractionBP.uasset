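; BridgeinteractionBP is a bridge interaction Blueprint that toggles the in-game visibility of three components, named 1, 2 and 3, through collision overlaps.
; BeginPlay hides all three components.
; Overlapping collision 2 or 3 reveals the matching component, while overlapping collision 1 sets component 1 hidden again, so this graph never reveals it.
; The overlaps do not filter by actor, and visibility changes do not propagate to children.
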(event OnComponentBeginOverlap(1콜리전)
  (params (OverlappedComponent :type Primitive%20Component%20Object%20Reference) (OtherActor :type Actor%20Object%20Reference) (OtherComp :type Primitive%20Component%20Object%20Reference) (OtherBodyIndex :type Integer) (bFromSweep :type Boolean) (SweepResult :type Hit%20Result%20Structure%20%28by%20ref%29))
  (Development|SetHiddeninGame (Variables|Default|Get1) true false))

(event OnComponentBeginOverlap(2콜리전)
  (params (OverlappedComponent :type Primitive%20Component%20Object%20Reference) (OtherActor :type Actor%20Object%20Reference) (OtherComp :type Primitive%20Component%20Object%20Reference) (OtherBodyIndex :type Integer) (bFromSweep :type Boolean) (SweepResult :type Hit%20Result%20Structure%20%28by%20ref%29))
  (Development|SetHiddeninGame (Variables|Default|Get2) false false))

(event OnComponentBeginOverlap(3콜리전)
  (params (OverlappedComponent :type Primitive%20Component%20Object%20Reference) (OtherActor :type Actor%20Object%20Reference) (OtherComp :type Primitive%20Component%20Object%20Reference) (OtherBodyIndex :type Integer) (bFromSweep :type Boolean) (SweepResult :type Hit%20Result%20Structure%20%28by%20ref%29))
  (Development|SetHiddeninGame (Variables|Default|Get3) false false))

(event EventBeginPlay
  (Utilities|FlowControl|Sequence
    (:then_0
      (Development|SetHiddeninGame (Variables|Default|Get1) true false))
    (:then_1
      (Development|SetHiddeninGame (Variables|Default|Get2) true false))
    (:then_2
      (Development|SetHiddeninGame (Variables|Default|Get3) true false))))

(fn ConstructionScript)