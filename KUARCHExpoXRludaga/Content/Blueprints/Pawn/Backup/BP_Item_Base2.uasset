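; Base Blueprint for a VR item that BP_VR_Hand can grip, hold, pass between hands and drop back into physics.
; Grip messages pick up the item or manipulate sub-components registered in SubComponentMap, snapping the hand mesh to a ghost hand and resetting parts on release.
; Trigger messages from the holding hand set Activated flags.
; Tick calls empty action functions for activation and manipulation, and highlight logic is disconnected.
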(event Custom|ItemPickedUp
  (params (Pawn :type Actor%20Object%20Reference) (Hand :type Actor%20Object%20Reference) (AttachPoint :type Scene%20Component%20Object%20Reference))
  (bind _asbp_vr_hand (Utilities|Casting|CastToBP_VR_Hand Hand))
  ;[1 1 1] Picked Up
  (CallFunction|PhysicsOff)
  (CallFunction|SetVarsforHand _asbp_vr_hand false)
  (CallFunction|SetLocalVars Pawn _asbp_vr_hand false)
  (CallFunction|SetHandOffset _asbp_vr_hand AttachPoint)
  (CallFunction|HandleAttachments AttachPoint))

(event Custom|ItemDropped
  ;[1 1 1] Dropped
  (Transformation|DetachFromActor "KeepWorld" "KeepWorld" "KeepWorld")
  (CallFunction|Physicson)
  (bind _keys (Utilities|Map|Keys (Variables|Default|GetSubComponentMap)))
  (for _array_element _keys
    (CallFunction|EndComponentManipulation _array_element))
  (bind _asbp_vr_hand (Utilities|Casting|CastToBP_VR_Hand (Variables|Default|GetOwningHand)))
  (CallFunction|SetVarsforHand _asbp_vr_hand true)
  (CallFunction|SetLocalVars 0 0 true))

(event Custom|StartComponentManipulation
  (params (OwningPawn :type Actor%20Object%20Reference) (OwningHand :type Actor%20Object%20Reference) (TargetComponent :type Scene%20Component%20Object%20Reference))
  (bind _subcomponentmap (Variables|Default|GetSubComponentMap))
  (bind (_value _returnvalue) (Utilities|Map|Find _subcomponentmap TargetComponent))
  (bind (_specificcomponent _basescene _highlighter _logicbp _maleattachments _femaleattachments _activated_ _anchor_ _ghosthand _manipulated_ _manipulatinghand _initialdistance _owningpawn) (Utilities|Struct|BreakStruct_ItemSubCompProperties _value))
  ;[1 1 1] Start Manipulation
  (if _returnvalue
    (|SetBy-RefVar _manipulated_ true)
    (|SetBy-RefVar _manipulatinghand (.AsBP%20VR%20Hand (Utilities|Casting|CastToBP_VR_Hand OwningHand)))
    (|SetBy-RefVar _owningpawn OwningPawn)
    (|SetBy-RefVar _initialdistance (Math|Vector|Distance(Vector) (Transformation|GetWorldLocation _specificcomponent) (Transformation|GetActorLocation _manipulatinghand)))
    (CallFunction|AttachHandtoMan _manipulatinghand _ghosthand)))

(event Custom|EndComponentManipulation
  (params (TargetComponent :type Scene%20Component%20Object%20Reference))
  (bind _subcomponentmap (Variables|Default|GetSubComponentMap))
  (bind (_value _returnvalue) (Utilities|Map|Find _subcomponentmap TargetComponent))
  (bind (_specificcomponent _basescene _highlighter _logicbp _maleattachments _femaleattachments _activated_ _anchor_ _activated__2 _manipulated_ _manipulatinghand _initialdistance _owningpawn _presettransformsrelative _presettarget) (Utilities|Struct|BreakStruct_ItemSubCompProperties _value))
  ;[1 1 1] End Manipulation
  (if _returnvalue
    (|SetBy-RefVar _manipulated_ false)
    (|SetBy-RefVar _activated__2 false)
    (|SetBy-RefVar _manipulatinghand)
    (|SetBy-RefVar _owningpawn)
    (|SetBy-RefVar _initialdistance 0.0)
    ;[1 1 1] Reset Component
    (Transformation|SetRelativeTransform _specificcomponent (Utilities|Array|Get(acopy) _presettransformsrelative _presettarget) false false)
    (Default|ResetMeshLocation _manipulatinghand)))

(event EventTick
  (params (DeltaSeconds :type Float%20%28single-precision%29))
  ;[1 1 1] Tick
  (Utilities|FlowControl|Sequence
    (:then_0
      ;[1 1 1] Call Item Activation
      (CallFunction|ActiveItemActions (Variables|Default|GetActivated?)))
    (:then_1
      (Utilities|FlowControl|Sequence
        (:then_0
          (bind _values (Utilities|Map|Values (Variables|Default|GetSubComponentMap)))
          (for _array_element _values
            (if (.Manipulated? (Utilities|Struct|BreakStruct_ItemSubCompProperties _array_element))
              (CallFunction|ManipulatedComponentActions _array_element))))))))

(event EventBeginPlay
  ;[1 1 1] Start
  (Utilities|FlowControl|Sequence
    (:then_0
      ;[1 1 1] Determine placement in hand when gripped
      (Variables|Default|SetHandOffset (Math|Transform|MakeTransform "9.000000,0.000000,-4.000000" "0.000000,540.000000,-180.000000" "1,1,1")))
    (:then_1
      (CallFunction|SetupComponents))))

(event EventHighlight
  (params (SpecificComponent :type Scene%20Component%20Object%20Reference)))

(event EventTrigger
  (params (Owner :type Actor%20Object%20Reference) (Hand :type Actor%20Object%20Reference) (Start0Stop1 :type Boolean) (SpecificComponent :type Scene%20Component%20Object%20Reference))
  (bind _subcomponentmap (Variables|Default|GetSubComponentMap))
  (bind (_value _returnvalue) (Utilities|Map|Find _subcomponentmap SpecificComponent))
  (bind _activated_ (Utilities|Struct|BreakStruct_ItemSubCompProperties _value))
  ;[1 1 1] Trigger Message
  (if (Variables|Default|GetHeld?)
    (if (== Hand (Variables|Default|GetOwningHand))
      ;[1 1 1] Base or Component?
      (if _returnvalue
        (if Start0Stop1
          (|SetBy-RefVar _activated_ false)
          (else
            (|SetBy-RefVar _activated_ true)))
        (elif Start0Stop1
          (Variables|Default|SetActivated? false)
          (else
            (Variables|Default|SetActivated? true)))))))

(event EventGrip
  (params (TargetComponent :type Scene%20Component%20Object%20Reference) (Owner :type Actor%20Object%20Reference) (Hand :type Actor%20Object%20Reference) (AttachPoint :type Scene%20Component%20Object%20Reference) (Start0End1 :type Boolean))
  (bind _subcomponentmap (Variables|Default|GetSubComponentMap))
  (bind (_value _returnvalue) (Utilities|Map|Find _subcomponentmap TargetComponent))
  (bind (_specificcomponent _basescene _highlighter _logicbp _maleattachments _femaleattachments _activated_ _anchor_ _manwohold_ _manipulatinghand) (Utilities|Struct|BreakStruct_ItemSubCompProperties _value))
  ;[1 1 1] Grip Message
  ;[1 1 1] Component or Whole Item?
  (if _returnvalue
    ;[1 1 1] Item Held?
    (if (Variables|Default|GetHeld?)
      ;[1 1 1] Held by same Pawn?
      (if (== Owner (Variables|Default|GetOwningPawn))
        ;[1 1 1] End or Start?
        (if Start0End1 :!label _label
          ;[1 1 1] Manipulating Hand?
          (if (== Hand _manipulatinghand)
            (CallFunction|EndComponentManipulation TargetComponent))
          (else
            (CallFunction|StartComponentManipulation Owner Hand TargetComponent))))
      (else
        ;[1 1 1] Manipulate with no Hold?
        (if _manwohold_
          (goto _label)
          (else
            ;[1 1 1] End or Start?
            (if Start0End1 :!label _label_2
              ;[1 1 1] Already Held by this Hand?
              (if (and (Variables|Default|GetHeld?) (== Hand (Variables|Default|GetOwningHand)))
                (CallFunction|ItemDropped :!label _label_3))
              (else
                ;[1 1 1] Already Held?
                (if (Variables|Default|GetHeld?)
                  ;[1 1 1] Release on Held+Start?
                  (if (Variables|Default|GetSticky?)
                    ;[1 1 1] Holding Hand?
                    (if (== Hand (Variables|Default|GetOwningHand))
                      (goto _label_3)
                      (else
                        _)))
                  ;[1 1 1] Held by Hand Owner?
                  (if (== Owner (Variables|Default|GetOwningPawn))
                    (CallFunction|ItemDropped :!label _label_4)
                    (CallFunction|ItemPickedUp Owner Hand AttachPoint))
                  (else
                    (goto _label_4)))))))))
    (else
      (goto _label_2))))

(event Custom|Component%20Manipulation
  (params (Target%20Component :type Scene%20Component%20Object%20Reference) (Manipulated? :type Boolean)))

(event Custom|ItemActivation
  (params (Activated? :type Boolean)))

(event Custom|ComponentActivation
  (params (Target%20Component :type Scene%20Component%20Object%20Reference) (Activated? :type Boolean)))

(fn ConstructionScript)

(fn AttachSelf
  (params (Parent :type Scene%20Component%20Object%20Reference) (Object :type Object%20Object%20Reference) (OwningPawn :type Actor%20Object%20Reference) (OwningHand :type Actor%20Object%20Reference))
  (bind _handoffset (Variables|Default|GetHandOffset))
  (bind (_roll _pitch _yaw) (Math|Rotator|BreakRotator (.rotation _handoffset)))
  (CallFunction|PhysicsOff)
  (Transformation|AttachComponentToComponent (Variables|Default|GetBaseMesh) (Variables|Default|GetDefaultSceneRoot) "None" "SnapToTarget" "SnapToTarget" "KeepWorld" true)
  (Transformation|AttachComponentToComponent Parent "None" "SnapToTarget" "SnapToTarget" "KeepWorld" true)
  (bind _asbp_vr_hand (Utilities|Casting|CastToBP_VR_Hand Object))
  (Variables|/Game/Blueprints/Pawn/BP_VR_Hand.BP_VR_Hand_C|SetHolding? _asbp_vr_hand true)
  (Variables|/Game/Blueprints/Pawn/BP_VR_Hand.BP_VR_Hand_C|SetHeldItem _asbp_vr_hand self)
  (Variables|Default|SetOwningPawn OwningPawn)
  (Variables|Default|SetOwningHand OwningHand)
  (Variables|Default|SetHeld? true)
  (if (Variables|/Game/Blueprints/Pawn/BP_VR_Hand.BP_VR_Hand_C|GetLeft0Rght1 _asbp_vr_hand)
    (Transformation|SetRelativeTransform (Variables|/Game/Blueprints/Pawn/BP_VR_Hand.BP_VR_Hand_C|GetAttachScene _asbp_vr_hand) (Math|Transform|MakeTransform (.location _handoffset) (.rotation _handoffset) "1,1,1") false false)
    (else
      (Transformation|SetRelativeTransform (Variables|/Game/Blueprints/Pawn/BP_VR_Hand.BP_VR_Hand_C|GetAttachScene _asbp_vr_hand) (Math|Transform|MakeTransform (.location _handoffset) (Math|Rotator|MakeRotator (+ _roll 1.8e+02) _pitch _yaw) "1,1,1") false false))))

(fn DetachSelf
  (params (Object :type Object%20Object%20Reference))
  (Transformation|DetachFromActor "KeepWorld" "KeepWorld" "KeepWorld")
  (bind _asbp_vr_hand (Utilities|Casting|CastToBP_VR_Hand Object)
    (:then
      (Variables|/Game/Blueprints/Pawn/BP_VR_Hand.BP_VR_Hand_C|SetHolding? _asbp_vr_hand false)
      (Variables|/Game/Blueprints/Pawn/BP_VR_Hand.BP_VR_Hand_C|SetHeldItem _asbp_vr_hand 0))
    (:CastFailed
      _))
  (Variables|Default|SetOwningPawn 0)
  (Variables|Default|SetOwningHand 0)
  (Variables|Default|SetHeld? false)
  (Transformation|AttachComponentToComponent (Variables|Default|GetBaseMesh) (Variables|Default|GetDefaultSceneRoot) "None" "SnapToTarget" "SnapToTarget" "KeepWorld" true)
  (CallFunction|Physicson))

(fn ChangeHands
  (bind _asbp_vr_hand (Utilities|Casting|CastToBP_VR_Hand (Variables|Default|GetOwningHand)))
  (Variables|/Game/Blueprints/Pawn/BP_VR_Hand.BP_VR_Hand_C|SetHolding? _asbp_vr_hand false)
  (Variables|/Game/Blueprints/Pawn/BP_VR_Hand.BP_VR_Hand_C|SetHeldItem _asbp_vr_hand 0))

(fn Physicson
  (bind _basemesh (Variables|Default|GetBaseMesh))
  (Physics|SetSimulatePhysics _basemesh true)
  (Physics|SetEnableGravity _basemesh true))

(fn PhysicsOff
  (bind _basemesh (Variables|Default|GetBaseMesh))
  (Physics|SetSimulatePhysics (Variables|Default|GetBaseHighlighter) false)
  (Physics|SetSimulatePhysics _basemesh false)
  (Physics|SetSimulatePhysics _basemesh false)
  (Physics|SetEnableGravity _basemesh false))

(fn ClearLocalManVariables
  (Variables|Default|SetManipulated? false)
  (Variables|Default|SetManipulatingHand 0)
  (Variables|Default|SetInitialManDistance 0.0))

(fn ClearHandManVariables
  (params (HandActor :type BP%20VR%20Hand%20Object%20Reference))
  (Variables|/Game/Blueprints/Pawn/BP_VR_Hand.BP_VR_Hand_C|SetManipulating HandActor false)
  (Variables|/Game/Blueprints/Pawn/BP_VR_Hand.BP_VR_Hand_C|SetManipulatedActor HandActor 0)
  (Variables|/Game/Blueprints/Pawn/BP_VR_Hand.BP_VR_Hand_C|SetManipulatedComponent HandActor 0))

(fn SetLocalManVariables
  (params (ManipulatingHand :type Actor%20Object%20Reference))
  (Variables|Default|SetManipulated? true)
  (Variables|Default|SetManipulatingHand ManipulatingHand)
  (Variables|Default|SetInitialManDistance (Math|Vector|Distance(Vector) (Transformation|GetWorldLocation (Variables|Default|GetMan1Mesh)) (Transformation|GetActorLocation ManipulatingHand))))

(fn SetHandManVariables
  (params (TargetHand :type BP%20VR%20Hand%20Object%20Reference) (ManipulatedComponent :type Scene%20Component%20Object%20Reference))
  (Variables|/Game/Blueprints/Pawn/BP_VR_Hand.BP_VR_Hand_C|SetManipulating TargetHand true)
  (Variables|/Game/Blueprints/Pawn/BP_VR_Hand.BP_VR_Hand_C|SetManipulatedActor TargetHand self)
  (Variables|/Game/Blueprints/Pawn/BP_VR_Hand.BP_VR_Hand_C|SetManipulatedComponent TargetHand ManipulatedComponent))

(fn AttachHandtoMan
  (params (HandActor :type BP%20VR%20Hand%20Object%20Reference) (Component :type Scene%20Component%20Object%20Reference))
  (bind _handmesh (Variables|/Game/Blueprints/Pawn/BP_VR_Hand.BP_VR_Hand_C|GetHandMesh HandActor))
  (Transformation|AttachComponentToComponent _handmesh Component "None" "SnapToTarget" "SnapToTarget" "KeepWorld" true)
  (if (not (Variables|/Game/Blueprints/Pawn/BP_VR_Hand.BP_VR_Hand_C|GetLeft0Rght1 HandActor))
    (Transformation|AddRelativeRotation _handmesh "0, 0,180.000000" false false)))

(fn ApplyHandOffset
  (params (HandActor :type BP%20VR%20Hand%20Object%20Reference))
  (bind _handoffset (Variables|Default|GetHandOffset))
  (bind _attachscene (Variables|/Game/Blueprints/Pawn/BP_VR_Hand.BP_VR_Hand_C|GetAttachScene HandActor))
  (bind (_roll _pitch _yaw) (Math|Rotator|BreakRotator (.rotation _handoffset)))
  (if (Variables|/Game/Blueprints/Pawn/BP_VR_Hand.BP_VR_Hand_C|GetLeft0Rght1 HandActor)
    (Transformation|SetRelativeTransform _attachscene (Math|Transform|MakeTransform (.location _handoffset) (.rotation _handoffset) "1,1,1") false false)
    (else
      (Transformation|SetRelativeTransform _attachscene (Math|Transform|MakeTransform (.location _handoffset) (Math|Rotator|MakeRotator (+ _roll 1.8e+02) _pitch _yaw) "1,1,1") false false))))

(fn HandleAttachments
  (params (Parent :type Scene%20Component%20Object%20Reference))
  ;[1 1 1] ReAttachMesh
  (Transformation|AttachComponentToComponent (Variables|Default|GetBaseMesh) (Variables|Default|GetDefaultSceneRoot) "None" "SnapToTarget" "SnapToTarget" "KeepWorld" true)
  ;[1 1 1] Attach Item to Hand at Scene
  (Transformation|AttachComponentToComponent Parent "None" "SnapToTarget" "SnapToTarget" "KeepWorld" true))

(fn SetVarsforHand
  (params (Hand%20Actor :type BP%20VR%20Hand%20Object%20Reference) (Clear? :type Boolean))
  (if Clear?
    (Variables|/Game/Blueprints/Pawn/BP_VR_Hand.BP_VR_Hand_C|SetHolding? Hand%20Actor false)
    (Variables|/Game/Blueprints/Pawn/BP_VR_Hand.BP_VR_Hand_C|SetHeldItem Hand%20Actor 0)
    (else
      (Variables|/Game/Blueprints/Pawn/BP_VR_Hand.BP_VR_Hand_C|SetHolding? Hand%20Actor true)
      (Variables|/Game/Blueprints/Pawn/BP_VR_Hand.BP_VR_Hand_C|SetHeldItem Hand%20Actor self))))

(fn SetLocalVars
  (params (OwningPawn :type Actor%20Object%20Reference) (OwningHand :type Actor%20Object%20Reference) (Clear? :type Boolean))
  (if Clear?
    (Variables|Default|SetOwningPawn 0)
    (Variables|Default|SetOwningHand 0)
    (Variables|Default|SetHeld? false)
    (else
      (Variables|Default|SetOwningPawn OwningPawn)
      (Variables|Default|SetOwningHand OwningHand)
      (Variables|Default|SetHeld? true))))

(fn SetHandOffset
  (params (HandActor :type BP%20VR%20Hand%20Object%20Reference) (Attach%20Point :type Scene%20Component%20Object%20Reference))
  (bind _handoffset (Variables|Default|GetHandOffset))
  (bind (_roll _pitch _yaw) (Math|Rotator|BreakRotator (.rotation _handoffset)))
  (if (Variables|/Game/Blueprints/Pawn/BP_VR_Hand.BP_VR_Hand_C|GetLeft0Rght1 HandActor)
    (Transformation|SetRelativeTransform Attach%20Point (Math|Transform|MakeTransform (.location _handoffset) (.rotation _handoffset) "1,1,1") false false)
    (else
      (Transformation|SetRelativeTransform Attach%20Point (Math|Transform|MakeTransform (.location _handoffset) (Math|Rotator|MakeRotator (+ _roll 1.8e+02) _pitch _yaw) "1,1,1") false false))))

(fn SetupComponents
  (bind _man2mesh (Variables|Default|GetMan2Mesh))
  (bind _man1mesh (Variables|Default|GetMan1Mesh))
  ;[1 1 1] SetupManComps
  (Utilities|FlowControl|Sequence
    (:then_0
      (Utilities|Map|Add (Variables|Default|GetSubComponentMap) _man1mesh (Utilities|Struct|MakeStruct_ItemSubCompProperties _man1mesh 0 (Variables|Default|GetMan1Highlighter) 0 "(MaleAttachable?_11_368F68E44450541CCEBFB3B54FB02ED7=False,TagTargets_16_2D9CC1914C1287BD23D04C97999008CB=(\"\"),MaleAttachLocationRefScene_18_6280FEEA4917F131C383DFB5047871A9=None,OnDropOnly?_3_7FC864CD458A1BAB7B2D86AB7FB2D84C=True,Preview?_5_472DC8E24FE12446631A9E82B8367E64=False,AttachedNow?_7_8879E57F46776D842CB8A68460A1C8B4=False)" "(FemaleAttachable?_12_368F68E44450541CCEBFB3B54FB02ED7=False,AcceptableTags_17_2D9CC1914C1287BD23D04C97999008CB=(\"\"),FemaleAttachLocationRefScene_19_A62D5BB74EB64D3BE5AFA799753E2972=None,AttachedNow?_7_8879E57F46776D842CB8A68460A1C8B4=False)" false false (Variables|Default|GetMan1HandGhost) (LocalVariables|GetN))))
    (:then_1
      (Utilities|Map|Add (Variables|Default|GetSubComponentMap) _man2mesh (Utilities|Struct|MakeStruct_ItemSubCompProperties _man2mesh 0 (Variables|Default|GetMan2Highlighter) 0 "(MaleAttachable?_11_368F68E44450541CCEBFB3B54FB02ED7=False,TagTargets_16_2D9CC1914C1287BD23D04C97999008CB=(\"\"),MaleAttachLocationRefScene_18_6280FEEA4917F131C383DFB5047871A9=None,OnDropOnly?_3_7FC864CD458A1BAB7B2D86AB7FB2D84C=True,Preview?_5_472DC8E24FE12446631A9E82B8367E64=False,AttachedNow?_7_8879E57F46776D842CB8A68460A1C8B4=False)" "(FemaleAttachable?_12_368F68E44450541CCEBFB3B54FB02ED7=False,AcceptableTags_17_2D9CC1914C1287BD23D04C97999008CB=(\"\"),FemaleAttachLocationRefScene_19_A62D5BB74EB64D3BE5AFA799753E2972=None,AttachedNow?_7_8879E57F46776D842CB8A68460A1C8B4=False)" false false (Variables|Default|GetMan2HandGhost) (LocalVariables|GetN)))))
  (LocalVariables|SetN (+ (LocalVariables|GetN) 1)))

(fn ActiveItemActions
  (params (Activated? :type Boolean)))

(fn ActiveComponentActions
  (params (TargetComponent :type Scene%20Component%20Object%20Reference) (Activated? :type Boolean)))

(fn ManipulatedComponentActions
  (params (Component%20Struct :type Struct%20Item%20Sub%20Comp%20Properties%20Structure%20%28by%20ref%29)))