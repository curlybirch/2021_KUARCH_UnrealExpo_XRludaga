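; VR hand actor that attaches to a motion controller and lets the player target, grip and use items.
; While empty-handed, Tick picks a target by priority: "man"-tagged components in the close capsule, nearby pickups, then unheld pickups in the far capsule.
; Pickup targets get a highlight message and show the matching capsule.
; Grip and trigger events only send interface messages; target objects decide the response and set the hand's state.
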(event Custom|SendGrip
  (params (Start0End1 :type Boolean))
  (bind _self self)
  (bind _owningpawn (Variables|Default|GetOwningPawn))
  (bind _pickuptarget (Variables|Default|GetPickupTarget))
  (bind _attachscene (Variables|Default|GetAttachScene))
  ;[1 1 1] Sends Request only, the object decides how to respond and sets relevant variables
  (if (Variables|Default|GetHolding?)
    ;[1 1 1] Send Grip Message to Held Item
    (Class|InterfacePickup|Grip(Message) (Variables|Default|GetHeldItem) 0 (Variables|Default|GetOwningPawn) self (Variables|Default|GetAttachScene) Start0End1)
    (else
      ;[1 1 1] Stop or Start?
      (if Start0End1
        (if (Variables|Default|GetManipulating)
          ;[1 1 1] Send End Manipulation Message
          (Class|InterfacePickup|Grip(Message) (Variables|Default|GetManipulatedActor) 0 _owningpawn _self _attachscene Start0End1 true (Variables|Default|GetManipulatedItem)))
        (else
          (Utilities|IsValid _pickuptarget
            (:Is%20Valid
              (if (Variables|Default|GetManTarget)
                ;[1 1 1] Send Begin Manipulate Message
                (Class|InterfacePickup|Grip(Message) (Variables|Default|GetPickupTarget) 0 _owningpawn _self _attachscene Start0End1 true (Variables|Default|GetManipulateTarget))
                (else
                  ;[1 1 1] Send Begin Grip Message
                  (Class|InterfacePickup|Grip(Message) _pickuptarget 0 _owningpawn _self _attachscene false))))))))))

(event Custom|SendTrigger
  (params (StartStop :type Boolean))
  (if (Variables|Default|GetHolding?)
    (Class|InterfacePickup|Trigger(Message) (Variables|Default|GetHeldItem) (Variables|Default|GetOwningPawn) self StartStop)))

(event Custom|ResetMeshLocation
  (bind _handmesh (Variables|Default|GetHandMesh))
  (Transformation|AttachComponentToComponent _handmesh (Variables|Default|GetDefaultSceneRoot) "None" "KeepRelative" "KeepRelative" "KeepWorld" true)
  (Transformation|SetRelativeLocationAndRotation _handmesh "-17.804718,-1.028018,5.748155" "-54.999859, 0,90.000000" false true)
  (if (not (Variables|Default|GetLeft0Rght1))
    (Transformation|SetWorldScale3D (Variables|Default|GetHandMesh) "1.000000,1.000000,-1.000000")))

(event EventBeginPlay
  (Utilities|FlowControl|Sequence
    (:then_0
      (Transformation|SetRelativeLocationAndRotation (Variables|Default|GetHandMesh) "-17.804718,-1.028018,5.748155" "-54.999859, 0,90.000000" false true)
      (if (not (Variables|Default|GetLeft0Rght1))
        (Transformation|SetWorldScale3D (Variables|Default|GetHandMesh) "1.000000,1.000000,-1.000000")))
    (:then_1
      (Transformation|AttachComponentToComponent (Variables|Default|GetController) "None" "SnapToTarget" "SnapToTarget" "KeepWorld" true))))

(event Collision|EventActorBeginOverlap
  (params (OtherActor :type Actor%20Object%20Reference)))

(event EventTick
  (params (DeltaSeconds :type Float%20%28single-precision%29))
  (Utilities|FlowControl|Sequence
    (:then_1
      (if (Variables|Default|GetHolding?)
        (CallFunction|ManageCapsuleVisibility true true)
        (else
          (CallFunction|ResetMans)
          (CallFunction|ResetPickups)
          ;[1 1 1] Look for close Manipulators
          (CallFunction|GetPotentialManipulators (Variables|Default|GetCloseCap))
          (if (Utilities|Array|IsValidIndex (Variables|Default|GetManipulatableComponents))
            ;[1 1 1] Prepare Manipulation
            (bind _closesttarget1 (CallFunction|FindClosestManipulator))
            (bind _output_get (Variables|Default|SetManipulateTarget _closesttarget1))
            (Variables|Default|SetPickupTarget (Components|GetOwner _output_get))
            (Variables|Default|SetManTarget true)
            (else
              (Variables|Default|SetManTarget false)
              ;[1 1 1] Look for close Pickups
              (CallFunction|GetPotentialPickups (Variables|Default|GetCloseCap) false)
              (if (Utilities|Array|IsValidIndex (Variables|Default|GetPickupableTargets))
                ;[1 1 1] Prepare Close PIckup
                (bind _closesttargetout (CallFunction|FindClosestTarget))
                (Variables|Default|SetPickupTarget _closesttargetout)
                (Utilities|IsValid (Variables|Default|GetPickupTarget)
                  (:Is%20Valid
                    (Class|InterfacePickup|Highlight(Message) (Variables|Default|GetPickupTarget))
                    (CallFunction|ManageCapsuleVisibility true false)))
                (else
                  (CallFunction|ResetPickups)
                  ;[1 1 1] Look for far Pickups
                  (CallFunction|GetPotentialPickups (Variables|Default|GetGrabCap) true)
                  (if (Utilities|Array|IsValidIndex (Variables|Default|GetPickupableTargets))
                    ;[1 1 1] Prepare Far Pickup
                    (bind _closesttargetout_2 (CallFunction|FindClosestTarget))
                    (Variables|Default|SetPickupTarget _closesttargetout_2)
                    (Utilities|IsValid (Variables|Default|GetPickupTarget)
                      (:Is%20Valid
                        (Class|InterfacePickup|Highlight(Message) (Variables|Default|GetPickupTarget))
                        (CallFunction|ManageCapsuleVisibility false true)))
                    (else
                      (CallFunction|ManageCapsuleVisibility true true))))))))))))

(fn ConstructionScript)

(fn MatchMotionControllerLocation
  (bind _defaultsceneroot (Variables|Default|GetDefaultSceneRoot))
  (bind _controller (Variables|Default|GetController))
  (Transformation|SetWorldTransform _defaultsceneroot (Math|Transform|MakeTransform (Math|Interpolation|VInterpTo (Transformation|GetWorldLocation _defaultsceneroot) (Transformation|GetWorldLocation _controller) (Utilities|Time|GetWorldDeltaSeconds) 6e+01) (Transformation|GetWorldRotation _controller) "1,1,1") false false))

(fn GetPotentialPickups
  (params (ScanCapsule :type Primitive%20Component%20Object%20Reference) (ExcludeHeld? :type Boolean))
  (bind _array_element (Utilities|Array|ForEachLoopwithBreak (Collision|GetOverlappingActors ScanCapsule "/Game/Blueprints/Interaction/BP_Item_Base.BP_Item_Base_C" :!class /Script/Engine.PrimitiveComponent))
    (:LoopBody
      (if (Utilities|DoesObjectImplementInterface _array_element "/Game/Blueprints/Helpers/Interface_Pickup.Interface_Pickup_C")
        (if ExcludeHeld?
          (if (not (Variables|/Game/Blueprints/Interaction/BP_Item_Base.BP_Item_Base_C|GetHeld? (.AsBP%20Item%20Base (Utilities|Casting|CastToBP_Item_Base _array_element))))
            (Utilities|Array|Add (Variables|Default|GetPickupableTargets) _array_element :!label _label))
          (else
            (goto _label)))))))

(fn FindClosestTarget
  (LocalVariables|SetClosestDistance 0.0)
  (LocalVariables|SetClosestTarget 0)
  (for _array_element (Variables|Default|GetPickupableTargets)
    (if (or (< (Math|Vector|Distance(Vector) (Transformation|GetActorLocation _array_element) (Transformation|GetWorldLocation (Variables|Default|GetHandMesh))) (LocalVariables|GetClosestDistance)) (== (LocalVariables|GetClosestTarget) 0))
      (LocalVariables|SetClosestDistance (Math|Vector|Distance(Vector) (Transformation|GetActorLocation _array_element) (Transformation|GetWorldLocation (Variables|Default|GetHandMesh))))
      (LocalVariables|SetClosestTarget _array_element)))
  (return (LocalVariables|GetClosestTarget)))

(fn GetPotentialManipulators
  (params (ScanCapsule :type Primitive%20Component%20Object%20Reference))
  (bind _array_element (Utilities|Array|ForEachLoopwithBreak (Class|PrimitiveComponent|GetOverlappingComponents ScanCapsule))
    (:LoopBody
      (if (Components|ComponentHasTag _array_element "man")
        (Utilities|Array|Add (Variables|Default|GetManipulatableComponents) _array_element)))))

(fn FindClosestManipulator
  (bind _returnvalue (Transformation|GetActorLocation))
  (bind _handmesh (Variables|Default|GetHandMesh))
  (bind _returnvalue_2 (Transformation|GetWorldLocation _handmesh))
  (bind _returnvalue_3 (Math|Vector|Distance(Vector) _returnvalue _returnvalue_2))
  (LocalVariables|SetClosestDistance 0.0)
  (LocalVariables|SetClosestTarget 0)
  (for _array_element (Variables|Default|GetManipulatableComponents)
    (if (or (< _returnvalue_3 (LocalVariables|GetClosestDistance)) (== (LocalVariables|GetClosestTarget) 0))
      (LocalVariables|SetClosestDistance _returnvalue_3)
      (LocalVariables|SetClosestTarget _array_element)))
  (return (LocalVariables|GetClosestTarget)))

(fn ManageCapsuleVisibility
  (params (GrabHidden? :type Boolean) (CloseHIdden? :type Boolean))
  (Development|SetHiddeninGame (Variables|Default|GetGrabCap) GrabHidden? false)
  (Development|SetHiddeninGame (Variables|Default|GetCloseCap) CloseHIdden? false))

(fn ResetMans
  (Variables|Default|SetManipulateTarget 0)
  (Utilities|Array|Clear (Variables|Default|GetManipulatableComponents)))

(fn ResetPickups
  (Variables|Default|SetPickupTarget 0)
  (Utilities|Array|Clear (Variables|Default|GetPickupableTargets)))

(fn PrepareManipulation
  (params (ManipulateTarget :type Scene%20Component%20Object%20Reference))
  (bind _output_get (Variables|Default|SetManipulateTarget ManipulateTarget))
  (Variables|Default|SetPickupTarget (Components|GetOwner _output_get))
  (Variables|Default|SetManTarget true))