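; Base VR item actor, designed to be held by one BP_VR_Hand and manipulated by the other, with highlight and trigger-activation feedback.
; Grip attaches the second hand's mesh to a ghost point, but a hardwired branch bypasses its sticky/slick pickup and drop logic.
; Attach/detach helpers toggle physics and apply mirrored hand offsets.
; Tick swaps state materials and queries a distance cutoff whose comparison is left unconnected.
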(event Custom|EndManipulation
  (params (HandActor :type BP%20VR%20Hand%20Object%20Reference))
  (CallFunction|ClearLocalManVariables)
  (CallFunction|ClearHandManVariables HandActor)
  (Default|ResetMeshLocation HandActor))

(event Custom|BeginManipulation
  (params (HandActor :type BP%20VR%20Hand%20Object%20Reference))
  (CallFunction|SetLocalManVariables HandActor)
  (CallFunction|SetHandManVariables HandActor)
  (CallFunction|AttachHandtoMan HandActor))

(event EventTick
  (params (DeltaSeconds :type Float%20%28single-precision%29))
  (bind _basemesh (Variables|Default|GetBaseMesh))
  (bind _man1mesh (Variables|Default|GetMan1Mesh))
  ;[1 1 1] Tick
  (Utilities|FlowControl|Sequence
    (:then_0
      ;[1 1 1] Activation Response Toggle
      (if (Variables|Default|GetActivated?)
        (Rendering|Material|SetMaterial _basemesh 0 "/Engine/VREditor/BasicMeshes/MI_Cube_02.MI_Cube_02")
        (else
          (Rendering|Material|SetMaterial _basemesh 0 "/Engine/VREditor/BasicMeshes/MI_Cube_03.MI_Cube_03"))))
    (:then_1
      ;[1 1 1] Manipulation Response Toggle
      (if (Variables|Default|GetManipulated?)
        (Rendering|Material|SetMaterial _man1mesh 0 "/Engine/VREditor/BasicMeshes/MI_Cube_02.MI_Cube_02")
        ;[1 1 1] Has the manipulating controller gotten too far away?
        (if (Utilities|AutoCutoffbyDistance 2.0)
          (CallFunction|EndManipulation (.AsBP%20VR%20Hand (Utilities|Casting|CastToBP_VR_Hand (Variables|Default|GetManipulatingHand)))))
        (else
          (Rendering|Material|SetMaterial _man1mesh 0 "/Engine/VREditor/BasicMeshes/MI_Cube_03.MI_Cube_03"))))))

(event EventHighlight
  (params (SpecificComponent :type Scene%20Component%20Object%20Reference))
  (if (not (Variables|Default|GetHeld?))
    (Development|SetHiddeninGame (Variables|Default|GetBaseHighlighter) false false)
    (Utilities|FlowControl|RetriggerableDelay 0.1)
    (Development|SetHiddeninGame (Variables|Default|GetBaseHighlighter) true false)))

(event EventTrigger
  (params (Owner :type Actor%20Object%20Reference) (Hand :type Actor%20Object%20Reference) (Start0Stop1 :type Boolean) (SpecificComponent :type Scene%20Component%20Object%20Reference))
  ;[1 1 1] Trigger Message
  (if (Variables|Default|GetHeld?)
    (if (== Hand (Variables|Default|GetOwningHand))
      (if Start0Stop1
        (Variables|Default|SetActivated? false)
        (else
          (Variables|Default|SetActivated? true))))))

(event EventGrip
  (params (TargetComponent :type Scene%20Component%20Object%20Reference) (Owner :type Actor%20Object%20Reference) (Hand :type Actor%20Object%20Reference) (AttachPoint :type Scene%20Component%20Object%20Reference) (Start0End1 :type Boolean))
  (bind _asbp_vr_hand (Utilities|Casting|CastToBP_VR_Hand Hand))
  ;[1 1 1] Grip Message
  (if true
    ;[1 1 1] Man Conditions
    (if (Math|Boolean|ANDBoolean (Variables|Default|GetHeld?) (== (Variables|Default|GetOwningPawn) Owner) (!= Hand (Variables|Default|GetOwningHand)))
      (if Start0End1
        ;[1 1 1] Manipulate
        (CallFunction|EndManipulation _asbp_vr_hand)
        (else
          (CallFunction|BeginManipulation _asbp_vr_hand))))
    (else
      ;[1 1 1] Drop on Release or Second Grip?
      (if (Variables|Default|GetSticky?)
        ;[1 1 1] Start or Stop Sticky
        (if (not Start0End1)
          (if (Variables|Default|GetHeld?)
            ;[1 1 1] Only Allow Owning Hand to drop
            (if (== Hand (Variables|Default|GetOwningHand)) :!label _label
              ;[1 1 1] Drop
              (CallFunction|DetachSelf Hand)
              (if (Variables|Default|GetManipulated?)
                ;[1 1 1] Give other hand back
                (CallFunction|EndManipulation (.AsBP%20VR%20Hand (Utilities|Casting|CastToBP_VR_Hand Hand)))))
            (else
              ;[1 1 1] PIckup
              (CallFunction|AttachSelf AttachPoint Hand Owner Hand :!label _label_2))))
        (else
          ;[1 1 1] Start or Stop Slick
          (if Start0End1
            (goto _label)
            (elif (Variables|Default|GetHeld?)
              ;[1 1 1] Allow only owner to switch hands
              (if (== Owner (Variables|Default|GetOwningPawn))
                (CallFunction|ChangeHands)
                (goto _label_2))
              (else
                (goto _label_2)))))))))

(event EventBeginPlay
  ;[1 1 1] Start
  (Utilities|FlowControl|Sequence
    (:then_0
      ;[1 1 1] Determine placement in hand when gripped
      (Variables|Default|SetHandOffset (Math|Transform|MakeTransform "9.000000,0.000000,-4.000000" "0.000000,540.000000,-180.000000" "1,1,1")))))

(fn ConstructionScript)

(fn AttachSelf
  (params (Parent :type Scene%20Component%20Object%20Reference) (Object :type Object%20Object%20Reference) (OwningPawn :type Actor%20Object%20Reference) (OwningHand :type Actor%20Object%20Reference))
  (bind _handoffset (Variables|Default|GetHandOffset))
  (bind (_roll _pitch _yaw) (Math|Rotator|BreakRotator (.rotation _handoffset)))
  (CallFunction|PhysicsOff)
  (Transformation|AttachComponentToComponent (Variables|Default|GetBaseMesh) (Variables|Default|GetDefaultSceneRoot) "None" "SnapToTarget" "SnapToTarget" "KeepWorld" true)
  (Transformation|AttachComponentToComponent Parent "None" "SnapToTarget" "SnapToTarget" "KeepWorld" true)
  (bind _asbp_vr_hand (Utilities|Casting|CastToBP_VR_Hand Object))
  (Variables|/Game/Blueprints/Pawn/BP_VR_Hand.BP_VR_Hand_C|SetHolding? _asbp_vr_hand true)
  (Variables|/Game/Blueprints/Pawn/BP_VR_Hand.BP_VR_Hand_C|SetHeldItem _asbp_vr_hand self)
  (Variables|Default|SetOwningPawn OwningPawn)
  (Variables|Default|SetOwningHand OwningHand)
  (Variables|Default|SetHeld? true)
  (if (Variables|/Game/Blueprints/Pawn/BP_VR_Hand.BP_VR_Hand_C|GetLeft0Rght1 _asbp_vr_hand)
    (Transformation|SetRelativeTransform (Variables|/Game/Blueprints/Pawn/BP_VR_Hand.BP_VR_Hand_C|GetAttachScene _asbp_vr_hand) (Math|Transform|MakeTransform (.location _handoffset) (.rotation _handoffset) "1,1,1") false false)
    (else
      (Transformation|SetRelativeTransform (Variables|/Game/Blueprints/Pawn/BP_VR_Hand.BP_VR_Hand_C|GetAttachScene _asbp_vr_hand) (Math|Transform|MakeTransform (.location _handoffset) (Math|Rotator|MakeRotator (+ _roll 1.8e+02) _pitch _yaw) "1,1,1") false false))))

(fn DetachSelf
  (params (Object :type Object%20Object%20Reference))
  (Transformation|DetachFromActor "KeepWorld" "KeepWorld" "KeepWorld")
  (bind _asbp_vr_hand (Utilities|Casting|CastToBP_VR_Hand Object)
    (:then
      (Variables|/Game/Blueprints/Pawn/BP_VR_Hand.BP_VR_Hand_C|SetHolding? _asbp_vr_hand false)
      (Variables|/Game/Blueprints/Pawn/BP_VR_Hand.BP_VR_Hand_C|SetHeldItem _asbp_vr_hand 0))
    (:CastFailed
      _))
  (Variables|Default|SetOwningPawn 0)
  (Variables|Default|SetOwningHand 0)
  (Variables|Default|SetHeld? false)
  (Transformation|AttachComponentToComponent (Variables|Default|GetBaseMesh) (Variables|Default|GetDefaultSceneRoot) "None" "SnapToTarget" "SnapToTarget" "KeepWorld" true)
  (CallFunction|Physicson))

(fn ChangeHands
  (bind _asbp_vr_hand (Utilities|Casting|CastToBP_VR_Hand (Variables|Default|GetOwningHand)))
  (Variables|/Game/Blueprints/Pawn/BP_VR_Hand.BP_VR_Hand_C|SetHolding? _asbp_vr_hand false)
  (Variables|/Game/Blueprints/Pawn/BP_VR_Hand.BP_VR_Hand_C|SetHeldItem _asbp_vr_hand 0))

(fn Physicson
  (bind _basemesh (Variables|Default|GetBaseMesh))
  (Physics|SetSimulatePhysics _basemesh true)
  (Physics|SetEnableGravity _basemesh true))

(fn PhysicsOff
  (bind _basemesh (Variables|Default|GetBaseMesh))
  (Physics|SetSimulatePhysics (Variables|Default|GetBaseHighlighter) false)
  (Physics|SetSimulatePhysics _basemesh false)
  (Physics|SetSimulatePhysics _basemesh false)
  (Physics|SetEnableGravity _basemesh false))

(fn ClearLocalManVariables
  (Variables|Default|SetManipulated? false)
  (Variables|Default|SetManipulatingHand 0)
  (Variables|Default|SetInitialManDistance 0.0))

(fn ClearHandManVariables
  (params (HandActor :type BP%20VR%20Hand%20Object%20Reference))
  (Variables|/Game/Blueprints/Pawn/BP_VR_Hand.BP_VR_Hand_C|SetManipulating HandActor false)
  (Variables|/Game/Blueprints/Pawn/BP_VR_Hand.BP_VR_Hand_C|SetManipulatedActor HandActor 0))

(fn SetLocalManVariables
  (params (ManipulatingHand :type Actor%20Object%20Reference))
  (Variables|Default|SetManipulated? true)
  (Variables|Default|SetManipulatingHand ManipulatingHand)
  (Variables|Default|SetInitialManDistance (Math|Vector|Distance(Vector) (Transformation|GetWorldLocation (Variables|Default|GetMan1Mesh)) (Transformation|GetActorLocation ManipulatingHand))))

(fn SetHandManVariables
  (params (TargetHand :type BP%20VR%20Hand%20Object%20Reference))
  (Variables|/Game/Blueprints/Pawn/BP_VR_Hand.BP_VR_Hand_C|SetManipulating TargetHand true)
  (Variables|/Game/Blueprints/Pawn/BP_VR_Hand.BP_VR_Hand_C|SetManipulatedActor TargetHand self))

(fn AttachHandtoMan
  (params (HandActor :type BP%20VR%20Hand%20Object%20Reference))
  (bind _handmesh (Variables|/Game/Blueprints/Pawn/BP_VR_Hand.BP_VR_Hand_C|GetHandMesh HandActor))
  (Transformation|AttachComponentToComponent _handmesh (Variables|Default|GetMan1HandGhost) "None" "SnapToTarget" "SnapToTarget" "KeepWorld" true)
  (if (not (Variables|/Game/Blueprints/Pawn/BP_VR_Hand.BP_VR_Hand_C|GetLeft0Rght1 HandActor))
    (Transformation|AddRelativeRotation _handmesh "0, 0,180.000000" false false)))

(fn ApplyHandOffset
  (params (HandActor :type BP%20VR%20Hand%20Object%20Reference))
  (bind _handoffset (Variables|Default|GetHandOffset))
  (bind _attachscene (Variables|/Game/Blueprints/Pawn/BP_VR_Hand.BP_VR_Hand_C|GetAttachScene HandActor))
  (bind (_roll _pitch _yaw) (Math|Rotator|BreakRotator (.rotation _handoffset)))
  (if (Variables|/Game/Blueprints/Pawn/BP_VR_Hand.BP_VR_Hand_C|GetLeft0Rght1 HandActor)
    (Transformation|SetRelativeTransform _attachscene (Math|Transform|MakeTransform (.location _handoffset) (.rotation _handoffset) "1,1,1") false false)
    (else
      (Transformation|SetRelativeTransform _attachscene (Math|Transform|MakeTransform (.location _handoffset) (Math|Rotator|MakeRotator (+ _roll 1.8e+02) _pitch _yaw) "1,1,1") false false))))