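; VR hand actor that handles gripping, triggering, manipulating, pointing and physical contact for the pawn.
; Each tick it picks the nearest manipulator, close pickup or far pickup, highlights it and poses the hand; grip and trigger messages route to targeted or held actors.
; When free, a ghost hand pushes physics bodies by hand velocity and box-traces static geometry, detaching the visible mesh to slide along blocking surfaces.
; Pointing presses tagged buttons.
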(event Custom|SendGrip
  (params (Start0End1 :type Boolean))
  ;[1 1 1] Grip Message
  (if (Variables|Default|GetUsing?)
    (Variables|Default|SetGripTargetActor (Variables|Default|GetUsedActor))
    (Variables|Default|SetGripTargetComponent (Variables|Default|GetUsedComponent))
    (elif Start0End1
      (Variables|Default|SetGrip false)
      (else
        (Variables|Default|SetGrip true))))
  (Class|InterfacePickup|Grip(Message) (Variables|Default|GetGripTargetActor) (Variables|Default|GetGripTargetComponent) (Variables|Default|GetOwningPawn) self (Variables|Default|GetAttachScene) Start0End1))

(event Custom|SendTrigger
  (params (StartStop :type Boolean))
  ;[1 1 1] Trigger Message
  (if (Variables|Default|GetUsing?)
    (Class|InterfacePickup|Trigger(Message) (Variables|Default|GetUsedActor) (Variables|Default|GetOwningPawn) self StartStop (Variables|Default|GetUsedComponent))
    (elif StartStop
      (Variables|Default|SetTrig false)
      (else
        (Variables|Default|SetTrig true)))))

(event Custom|ResetMeshLocation
  ;[1 1 1] Called by Item on Drop
  (CallFunction|ReAttach)
  (CallFunction|ResetTransform))

(event Custom|AnchorGripped
  (params (SubComponentStruct :type Struct%20Item%20Sub%20Comp%20Properties%20Structure%20%28by%20ref%29) (Start0Stop1 :type Boolean))
  ;[1 1 1] Anchor Message
  (Default|AnchorPawn (.AsBP%20VR%20Pawn (Utilities|Casting|CastToBP_VR_Pawn (Variables|Default|GetOwningPawn))) Start0Stop1 (Variables|Default|GetController) SubComponentStruct))

(event Custom|HandChangeOverride
  (params (GripTarget :type GripTargetEnum%20Enum :default "NewEnumerator0") (GripOveride :type Float%20%28single-precision%29))
  ;[1 1 1] Hand Animation Var Message
  (Default|ChangeOverride (.AsRight%20Hand%20Anim%20BP (Utilities|Casting|CastToRightHand_AnimBP (Components|SkeletalMesh|GetAnimInstance (Variables|Default|GetHandMesh)))) GripTarget GripOveride)
  (Default|ChangeOverride (.AsRight%20Hand%20Anim%20BP (Utilities|Casting|CastToRightHand_AnimBP (Components|SkeletalMesh|GetAnimInstance (Variables|Default|GetPawnGhostHand)))) GripTarget GripOveride))

(event EventBeginPlay
  ;[1 1 1] Start
  (Utilities|FlowControl|Sequence
    (:then_0
      (CallFunction|ResetTransform))
    (:then_1
      (Transformation|AttachComponentToComponent (Variables|Default|GetController) "None" "SnapToTarget" "SnapToTarget" "KeepWorld" true))
    (:then_2
      (bind _outactors (Actor|GetAllActorsOfClass "/Game/Blueprints/Interaction/Widget_Actor.Widget_Actor_C"))
      (Variables|Default|SetWidget_Ref (Utilities|Array|Get(acopy) _outactors)))))

(event EventTick
  (params (DeltaSeconds :type Float%20%28single-precision%29))
  ;[1 1 1] Tick
  (Utilities|FlowControl|Sequence
    (:then_0
      (CallFunction|HandModeSelection))
    (:then_1
      (CallFunction|FindItemTargets))
    (:then_2
      (CallFunction|HandPhysics))))

(event Input|ActionEvents|InputActionLeftFaceAPress
  (params (Key :type Key%20Structure :default "None"))
  (bind _widgetinteraction (Variables|Default|GetWidgetInteraction))
  (:Pressed
    (Variables|/Script/UMG.WidgetInteractionComponent|SetbShowDebug _widgetinteraction false))
  (:Released
    (Variables|/Script/UMG.WidgetInteractionComponent|SetbShowDebug _widgetinteraction true)))

(event Input|ActionEvents|InputActionLeftFaceBPress
  (params (Key :type Key%20Structure :default "None"))
  (bind _widgetinteraction (Variables|Default|GetWidgetInteraction))
  (:Pressed
    (Class|WidgetInteractionComponent|PressPointerKey _widgetinteraction "LeftMouseButton"))
  (:Released
    (Class|WidgetInteractionComponent|ReleasePointerKey _widgetinteraction "LeftMouseButton")))

(event Input|KeyboardEvents|SpaceBar
  (params (Key :type Key%20Structure :default "None"))
  (bind _widgetinteraction (Variables|Default|GetWidgetInteraction))
  (:Pressed
    (Variables|/Script/UMG.WidgetInteractionComponent|SetbShowDebug _widgetinteraction false))
  (:Released
    (Variables|/Script/UMG.WidgetInteractionComponent|SetbShowDebug _widgetinteraction true)))

(event Custom|FindItemTargets
  (Utilities|FlowControl|Sequence
    (:then_0
      (if (Variables|Default|GetManipulating)
        (Variables|Default|SetUsing? true)
        (Variables|Default|SetUsedActor (Variables|Default|GetManipulatedActor))
        (Variables|Default|SetUsedComponent (Variables|Default|GetManipulatedComponent))
        (elif (Variables|Default|GetHolding?)
          (Variables|Default|SetUsing? true)
          (Variables|Default|SetUsedActor (Variables|Default|GetHeldItem))
          (Variables|Default|SetUsedComponent 0)
          (else
            (Variables|Default|SetUsing? false)
            (Variables|Default|SetUsedActor 0)))))
    (:then_1
      (if (Variables|Default|GetUsing?)
        (CallFunction|ManageCapsuleVisibility true true true)
        (else
          (CallFunction|ManageCapsuleVisibility true true true)
          (CallFunction|HandChangeOverride "NewEnumerator0" 0.0)
          (CallFunction|ResetMans)
          (CallFunction|ResetPickups)
          ;[1 1 1] Look for close Manipulators
          (CallFunction|GetPotentialManipulators (Variables|Default|GetCloseCap))
          (if (Utilities|Array|IsValidIndex (Variables|Default|GetManipulatableComponents))
            ;[1 1 1] Prepare Manipulation
            (bind _closesttarget1 (CallFunction|FindClosestManipulator))
            (bind _output_get (Variables|Default|SetGripTargetComponent _closesttarget1))
            (bind _output_get_2 (Variables|Default|SetGripTargetActor (Components|GetOwner _output_get)))
            (Class|InterfacePickup|Highlight(Message) _output_get_2 _output_get)
            (CallFunction|ManageCapsuleVisibility true true false)
            (CallFunction|HandChangeOverride "NewEnumerator1" 0.5)
            (Variables|Default|SetShouldDelaySearch false)
            ;[1 1 1] If no targets for a while, reduce search frequency
            (Utilities|FlowControl|RetriggerableDelay 0.3 :!label _label)
            (Variables|Default|SetShouldDelaySearch true)
            (else
              ;[1 1 1] Look for close Pickups
              (CallFunction|GetPotentialPickups (Variables|Default|GetCloseCap) false)
              (if (Utilities|Array|IsValidIndex (Variables|Default|GetPickupableTargets))
                ;[1 1 1] Prepare Close Pickup
                (bind _closesttargetout (CallFunction|FindClosestTarget))
                (Variables|Default|SetGripTargetComponent 0)
                (Variables|Default|SetGripTargetActor _closesttargetout)
                (Utilities|IsValid (Variables|Default|GetGripTargetActor)
                  (:Is%20Valid
                    (Class|InterfacePickup|Highlight(Message) (Variables|Default|GetGripTargetActor))
                    (CallFunction|ManageCapsuleVisibility true false true)
                    (CallFunction|HandChangeOverride "NewEnumerator1" 0.5)
                    (Variables|Default|SetShouldDelaySearch false)
                    (goto _label)))
                (else
                  (CallFunction|ResetPickups)
                  ;[1 1 1] Look for far Pickups
                  (CallFunction|GetPotentialPickups (Variables|Default|GetGrabCap) true)
                  (if (Utilities|Array|IsValidIndex (Variables|Default|GetPickupableTargets))
                    ;[1 1 1] Prepare Far Pickup
                    (bind _closesttargetout_2 (CallFunction|FindClosestTarget))
                    (Variables|Default|SetGripTargetActor _closesttargetout_2)
                    (Variables|Default|SetGripTargetComponent 0)
                    (Utilities|IsValid (Variables|Default|GetGripTargetActor)
                      (:Is%20Valid
                        (Class|InterfacePickup|Highlight(Message) (Variables|Default|GetGripTargetActor))
                        (CallFunction|ManageCapsuleVisibility false true true)
                        (CallFunction|HandChangeOverride "NewEnumerator1" 0.5)
                        (Variables|Default|SetShouldDelaySearch false)
                        (goto _label)))
                    (else
                      (Utilities|FlowControl|Sequence
                        (:then_0
                          (CallFunction|ManageCapsuleVisibility true true true))))))))))))))

(event OnComponentBeginOverlap(PawnGhostHand)
  (params (OverlappedComponent :type Primitive%20Component%20Object%20Reference) (OtherActor :type Actor%20Object%20Reference) (OtherComp :type Primitive%20Component%20Object%20Reference) (OtherBodyIndex :type Integer) (bFromSweep :type Boolean) (SweepResult :type Hit%20Result%20Structure%20%28by%20ref%29))
  (switch Utilities|FlowControl|Switch|SwitchonECollisionChannel (Collision|GetCollisionObjectType OtherComp)
    (:ECC_PhysicsBody
      (if (Physics|IsSimulatingPhysics OtherComp "None")
        ;[1 1 1] Impulse to Item
        (CallFunction|OneWayPhysics OtherComp)))))

(event OnComponentEndOverlap(PawnGhostHand)
  (params (OverlappedComponent :type Primitive%20Component%20Object%20Reference) (OtherActor :type Actor%20Object%20Reference) (OtherComp :type Primitive%20Component%20Object%20Reference) (OtherBodyIndex :type Integer)))

(event Custom|HandPhysics
  (Utilities|FlowControl|Sequence
    (:then_0
      (switch Utilities|FlowControl|Switch|SwitchonHandPhysEnum (Variables|Default|GetHandCollision)
        (:NewEnumerator0
          (Variables|Default|SetBlocked? false))
        (:NewEnumerator1
          ;[1 1 1] For Force to PhysicsBody
          (CallFunction|HandVelocityCalculation :!label _label))
        (:NewEnumerator2
          (bind _far_socket (CallFunction|SocketSelect :!label _label_2))
          ;[1 1 1] Block World Static
          (bind (_outhit _hit_) (CallFunction|CheckStaticBlock _far_socket))
          ;[1 1 1] HIT?
          (if _hit_
            (Variables|Default|SetBlocked? true)
            ;[1 1 1] Detach Mesh, Save Hit Info
            (CallFunction|BlockHand _outhit)
            (else
              (Variables|Default|SetBlocked? false))))
        (:NewEnumerator3
          (Utilities|FlowControl|Sequence
            (:then_0
              (goto _label))
            (:then_1
              (goto _label_2))))))
    (:then_1
      ;[1 1 1] PlaneSlide
      (if (Variables|Default|GetBlocked?)
        (Utilities|SlideonPlane _far_socket)
        (goto _label_3 Reset)
        (else
          ;[1 1 1] Give Hand back when not blocked
          (Utilities|FlowControl|DoOnce false :!label _label_3
            (:Completed
              (CallFunction|ResetMeshLocation))))))))

(event Custom|HandModeSelection
  (Utilities|FlowControl|Sequence
    (:then_0
      (Utilities|MakeFist?))
    (:then_1
      ;[1 1 1] Actions when Grip+Trigger
      (if (Variables|Default|GetUsing?)
        ;[1 0 0.7455] Temporary Debugging
        (Rendering|Material|SetMaterial (Variables|Default|GetHandMesh) 0 "/Game/VirtualReality/Mannequin/Character/Materials/M_HandMat.M_HandMat")
        ;[1 1 1] Physics Mode
        (CallFunction|SetHandPhysicsMode "NewEnumerator0")
        (else
          (Utilities|FlowControl|Delay 0.2)
          (Rendering|Material|SetMaterial (Variables|Default|GetHandMesh) 0 "/DatasmithContent/Materials/AliasMaster.AliasMaster")
          (CallFunction|SetHandPhysicsMode "NewEnumerator3"))))
    (:then_2
      ;[1 1 1] Set Pointing?
      (if (and (>= (Variables|Default|GetHandgrip) 0.25) (<= (Variables|Default|GetHandtrig) 0.5))
        (Variables|Default|SetPointing? true)
        (Variables|Default|SetScanY 0.0)
        (Variables|Default|SetScanZ 0.0)
        ;[1 1 1] Activate Buttons
        (for _array_element (Class|PrimitiveComponent|GetOverlappingComponents (Variables|Default|GetPointCap))
          (if (Components|ComponentHasTag _array_element "button")
            (bind _asbp_item_base (Utilities|Casting|CastToBP_Item_Base (Components|GetOwner _array_element)))
            (Default|ButtonFinger (.LogicBP (Utilities|Struct|BreakStruct_ItemSubCompProperties (.Value (Utilities|Map|Find (Variables|/Game/Blueprints/Interaction/BP_Item_Base.BP_Item_Base_C|GetSubComponentMap _asbp_item_base) _array_element)))) (Transformation|GetSocketLocation (Variables|Default|GetHandMesh) "pointsock"))))
        (else
          (Variables|Default|SetPointing? false)
          (Variables|Default|SetScanY 4.0)
          (Variables|Default|SetScanZ 3.0))))))

(fn ConstructionScript)

(fn MatchMotionControllerLocation
  (bind _defaultsceneroot (Variables|Default|GetDefaultSceneRoot))
  (bind _controller (Variables|Default|GetController))
  (Transformation|SetWorldTransform _defaultsceneroot (Math|Transform|MakeTransform (Math|Interpolation|VInterpTo (Transformation|GetWorldLocation _defaultsceneroot) (Transformation|GetWorldLocation _controller) (Utilities|Time|GetWorldDeltaSeconds) 6e+01) (Transformation|GetWorldRotation _controller) "1,1,1") false false))

(fn GetPotentialPickups
  (params (ScanCapsule :type Primitive%20Component%20Object%20Reference) (ExcludeHeld? :type Boolean))
  (bind _array_element (Utilities|Array|ForEachLoopwithBreak (Collision|GetOverlappingActors ScanCapsule "/Game/Blueprints/Interaction/BP_Item_Base.BP_Item_Base_C" :!class /Script/Engine.PrimitiveComponent))
    (:LoopBody
      (if (Utilities|DoesObjectImplementInterface _array_element "/Game/Blueprints/Helpers/Interface_Pickup.Interface_Pickup_C")
        (if ExcludeHeld?
          (if (not (Variables|/Game/Blueprints/Interaction/BP_Item_Base.BP_Item_Base_C|GetHeld? (.AsBP%20Item%20Base (Utilities|Casting|CastToBP_Item_Base _array_element))))
            (if (Variables|/Game/Blueprints/Interaction/BP_Item_Base.BP_Item_Base_C|GetHung? (.AsBP%20Item%20Base (Utilities|Casting|CastToBP_Item_Base _array_element)))
              (if (Variables|/Game/Blueprints/Interaction/BP_Item_Base.BP_Item_Base_C|GetPreferParentPickup? (.AsBP%20Item%20Base (Utilities|Casting|CastToBP_Item_Base _array_element)))
                (if (not (Variables|/Game/Blueprints/Interaction/BP_Item_Base.BP_Item_Base_C|GetHeld? (Variables|/Game/Blueprints/Interaction/BP_Item_Base.BP_Item_Base_C|GetParentItem (.AsBP%20Item%20Base (Utilities|Casting|CastToBP_Item_Base _array_element)))))
                  (if (not (Variables|/Game/Blueprints/Interaction/BP_Item_Base.BP_Item_Base_C|GetStayPut? (.AsBP%20Item%20Base (Utilities|Casting|CastToBP_Item_Base _array_element)))) :!label _label
                    (Utilities|Array|Add (Variables|Default|GetPickupableTargets) _array_element))))
              (else
                (goto _label))))
          (else
            (goto _label)))))))

(fn FindClosestTarget
  (LocalVariables|SetClosestDistance 0.0)
  (LocalVariables|SetClosestTarget 0)
  (for _array_element (Variables|Default|GetPickupableTargets)
    (if (or (< (Math|Vector|Distance(Vector) (Transformation|GetActorLocation _array_element) (Transformation|GetWorldLocation (Variables|Default|GetHandMesh))) (LocalVariables|GetClosestDistance)) (== (LocalVariables|GetClosestTarget) 0))
      (LocalVariables|SetClosestDistance (Math|Vector|Distance(Vector) (Transformation|GetActorLocation _array_element) (Transformation|GetWorldLocation (Variables|Default|GetHandMesh))))
      (LocalVariables|SetClosestTarget _array_element)))
  (return (LocalVariables|GetClosestTarget)))

(fn GetPotentialManipulators
  (params (ScanCapsule :type Primitive%20Component%20Object%20Reference))
  (bind _array_element (Utilities|Array|ForEachLoopwithBreak (Class|PrimitiveComponent|GetOverlappingComponents ScanCapsule))
    (:LoopBody
      (if (Components|ComponentHasTag _array_element "man")
        (Utilities|Array|Add (Variables|Default|GetManipulatableComponents) _array_element)))))

(fn FindClosestManipulator
  (bind _returnvalue (Transformation|GetActorLocation))
  (bind _handmesh (Variables|Default|GetHandMesh))
  (bind _returnvalue_2 (Transformation|GetWorldLocation _handmesh))
  (bind _returnvalue_3 (Math|Vector|Distance(Vector) _returnvalue _returnvalue_2))
  (LocalVariables|SetClosestDistance 0.0)
  (LocalVariables|SetClosestTarget 0)
  (for _array_element (Variables|Default|GetManipulatableComponents)
    (if (or (< _returnvalue_3 (LocalVariables|GetClosestDistance)) (== (LocalVariables|GetClosestTarget) 0))
      (LocalVariables|SetClosestDistance _returnvalue_3)
      (LocalVariables|SetClosestTarget _array_element)))
  (return (LocalVariables|GetClosestTarget)))

(fn ManageCapsuleVisibility
  (params (GrabHidden? :type Boolean) (CloseHIdden? :type Boolean) (ManHidden? :type Boolean)))

(fn ResetMans
  (Variables|Default|SetManipulateTarget 0)
  (Utilities|Array|Clear (Variables|Default|GetManipulatableComponents)))

(fn ResetPickups
  (Variables|Default|SetGripTargetActor 0)
  (Utilities|Array|Clear (Variables|Default|GetPickupableTargets)))

(fn PrepareManipulation
  (params (ManipulateTarget :type Scene%20Component%20Object%20Reference))
  (bind _output_get (Variables|Default|SetManipulateTarget ManipulateTarget))
  (Variables|Default|SetGripTargetActor (Components|GetOwner _output_get))
  (Variables|Default|SetManTarget true))

(fn ResetTransform
  (Transformation|SetRelativeLocationAndRotation (Variables|Default|GetHandMesh) (Variables|Default|GetHandLoc) (Variables|Default|GetHandRot) false true)
  (if (not (Variables|Default|GetLeft0Rght1))
    (Transformation|SetWorldScale3D (Variables|Default|GetHandMesh) "1.000000,1.000000,-1.000000")))

(fn ReAttach
  (Transformation|AttachComponentToComponent (Variables|Default|GetHandMesh) (Variables|Default|GetDefaultSceneRoot) "None" "KeepRelative" "KeepRelative" "KeepWorld" true)
  (return))

(fn SetHandPhysicsMode
  (params (Physics%20Type :type HandPhysEnum%20Enum :default "NewEnumerator0"))
  (bind _pawnghosthand (Variables|Default|GetPawnGhostHand))
  (Variables|Default|SetHandCollision Physics%20Type)
  (switch Utilities|FlowControl|Switch|SwitchonHandPhysEnum Physics%20Type
    (:NewEnumerator0
      (Collision|SetCollisionEnabled _pawnghosthand "NoCollision")
      (Collision|SetCollisionResponsetoChannel _pawnghosthand "ECC_PhysicsBody" "ECR_Ignore")
      (Collision|SetCollisionResponsetoChannel _pawnghosthand "ECC_WorldStatic" "ECR_Ignore"))
    (:NewEnumerator1
      (Collision|SetCollisionEnabled _pawnghosthand "QueryOnly")
      (Collision|SetCollisionResponsetoChannel _pawnghosthand "ECC_PhysicsBody" "ECR_Overlap")
      (Collision|SetCollisionResponsetoChannel _pawnghosthand "ECC_WorldStatic" "ECR_Ignore"))
    (:NewEnumerator2
      (Collision|SetCollisionEnabled _pawnghosthand "QueryOnly")
      (Collision|SetCollisionResponsetoChannel _pawnghosthand "ECC_WorldStatic" "ECR_Overlap")
      (Collision|SetCollisionResponsetoChannel _pawnghosthand "ECC_PhysicsBody" "ECR_Ignore"))
    (:NewEnumerator3
      (Collision|SetCollisionEnabled _pawnghosthand "QueryOnly")
      (Collision|SetCollisionResponsetoChannel _pawnghosthand "ECC_PhysicsBody" "ECR_Overlap")
      (Collision|SetCollisionResponsetoChannel _pawnghosthand "ECC_WorldStatic" "ECR_Overlap"))))

(fn OneWayPhysics
  (params (Target%20Component :type Primitive%20Component%20Object%20Reference))
  (Class|PrimitiveComponent|AddForceatLocation Target%20Component (* (* (Variables|Default|GetFrameVel) (/ 1.0 (Utilities|Time|GetWorldDeltaSeconds))) 5e+01) (Transformation|GetWorldLocation (Variables|Default|GetCloseCap)) "None"))

(fn HandVelocityCalculation
  (bind _closecap (Variables|Default|GetCloseCap))
  (bind _returnvalue (Transformation|GetWorldLocation _closecap))
  (bind _output_get (Variables|Default|SetCurrentLoc _returnvalue))
  (Variables|Default|SetFrameVel (- _output_get (Variables|Default|GetLastLoc)))
  (Variables|Default|SetLastLoc _returnvalue))

(fn BlockHand
  (params (Hit :type Hit%20Result%20Structure%20%28by%20ref%29) (Target%20Component :type Scene%20Component%20Object%20Reference))
  (bind (_bblockinghit _binitialoverlap _time _distance _location _impactpoint _normal) (Collision|BreakHitResult Hit))
  (Transformation|DetachFromComponent (Variables|Default|GetHandMesh) "KeepWorld" "KeepWorld" "KeepWorld" true)
  (Variables|Default|SetBlockPoint _location)
  (bind _output_get (Variables|Default|SetBlockNormal _normal))
  (Utilities|FlowControl|Sequence
    (:then_0
      (if (Math|Float|NearlyEqual(Float) (.X (Math|Vector|BreakVector _output_get)) 0.0 0.1)
        (|SetBy-RefVar _output_get (Math|Vector|MakeVector 0.0 (.Y (Math|Vector|BreakVector _output_get)) (.Z (Math|Vector|BreakVector _output_get))))))
    (:then_1
      (if (Math|Float|NearlyEqual(Float) (.Y (Math|Vector|BreakVector _output_get)) 0.0 0.1)
        (|SetBy-RefVar _output_get (Math|Vector|MakeVector (.X (Math|Vector|BreakVector _output_get)) 0.0 (.Z (Math|Vector|BreakVector _output_get))))))
    (:then_2
      (if (Math|Float|NearlyEqual(Float) (.Z (Math|Vector|BreakVector _output_get)) 0.0 0.1)
        (|SetBy-RefVar _output_get (Math|Vector|MakeVector (.X (Math|Vector|BreakVector _output_get)) (.Y (Math|Vector|BreakVector _output_get)) 0.0))))))

(fn CheckStaticBlock
  (params (End :type Vector))
  (bind _pawnghosthand (Variables|Default|GetPawnGhostHand))
  ;[1 1 1] Trace from Wrist to Finger Tip
  (bind (_outhit _returnvalue) (Class|KismetSystemLibrary|BoxTraceSingleforObjects (Transformation|GetSocketLocation _pawnghosthand "wristsock") End (Math|Vector|MakeVector 0.0 (Variables|Default|GetScanY) (Variables|Default|GetScanZ)) (Transformation|GetWorldRotation _pawnghosthand) (Utilities|Array|MakeArray "ObjectTypeQuery1") false 0 "None" true))
  (return _outhit _returnvalue))

(fn SocketSelect
  (bind _pawnghosthand (Variables|Default|GetPawnGhostHand))
  (LocalVariables|SetF_Distance 0.0)
  (for _array_element (Transformation|GetAllSocketNames _pawnghosthand)
    (if (>= (Math|Vector|Distance(Vector) (Transformation|GetSocketLocation (Variables|Default|GetPawnGhostHand) "wristsock") (Transformation|GetSocketLocation _pawnghosthand _array_element)) (LocalVariables|GetF_Distance))
      (LocalVariables|SetF_Distance (Math|Vector|Distance(Vector) (Transformation|GetSocketLocation (Variables|Default|GetPawnGhostHand) "wristsock") (Transformation|GetSocketLocation _pawnghosthand _array_element)))
      (LocalVariables|SetF_Location (Transformation|GetSocketLocation _pawnghosthand _array_element))))
  (return (LocalVariables|GetF_Location)))