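; Blueprint function library that converts between Cartesian grid positions (XYZ) and spherical coordinates stored as Radius, Azimuth and Inclination.
; Both directions use degree-based trig, with azimuth measured from +X in the XY plane and inclination from +Z.
; The FixedR variant keeps the computed angles but returns a supplied radius, projecting a point onto a sphere of that size.
; Neither grid-to-polar function guards against division by a zero radius.
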(fn ConvertGridtoPolar
  (params (GridXYZ :type Vector))
  (Utilities|FlowControl|Sequence
    (:then_0
      (LocalVariables|SetgX (.x GridXYZ))
      (LocalVariables|SetgY (.y GridXYZ))
      (LocalVariables|SetgZ (.z GridXYZ)))
    (:then_1
      (Utilities|FlowControl|Sequence
        (:then_0
          (LocalVariables|Setradius (Math|Float|Sqrt (+ (Math|Float|Square (LocalVariables|GetgX)) (Math|Float|Square (LocalVariables|GetgY)) (Math|Float|Square (LocalVariables|GetgZ))))))
        (:then_1
          (LocalVariables|Setazimuth (Class|KismetMathLibrary|DegAtan2 (LocalVariables|GetgY) (LocalVariables|GetgX))))
        (:then_2
          (LocalVariables|Setinclination (Class|KismetMathLibrary|DegAcos (/ (LocalVariables|GetgZ) (LocalVariables|Getradius)))))))
    (:then_2
      (return (Utilities|Struct|MakeSphereCoordsStruct (LocalVariables|Getradius) (LocalVariables|Getazimuth) (LocalVariables|Getinclination))))))

(fn ConvertPolartoGrid
  (params (PolarRAI :type Sphere%20Coords%20Struct%20Structure))
  (Utilities|FlowControl|Sequence
    (:then_0
      (LocalVariables|Setradius (.radius PolarRAI))
      (LocalVariables|Setazimuth (.azimuth PolarRAI))
      (LocalVariables|Setinclination (.inclination PolarRAI)))
    (:then_1
      (Utilities|FlowControl|Sequence
        (:then_0
          (LocalVariables|Setx (* (LocalVariables|Getradius) (Math|Trig|Sin(Degrees) (LocalVariables|Getinclination)) (Math|Trig|Cos(Degrees) (LocalVariables|Getazimuth)))))
        (:then_1
          (LocalVariables|Sety (* (LocalVariables|Getradius) (Math|Trig|Sin(Degrees) (LocalVariables|Getinclination)) (Math|Trig|Sin(Degrees) (LocalVariables|Getazimuth)))))
        (:then_2
          (LocalVariables|Setz (* (LocalVariables|Getradius) (Math|Trig|Cos(Degrees) (LocalVariables|Getinclination)))))))
    (:then_2
      (return (Math|Vector|MakeVector (LocalVariables|Getx) (LocalVariables|Gety) (LocalVariables|Getz))))))

(fn ConvertGridtoPolarFixedR
  (params (GridXYZ :type Vector) (SetRadius :type Float%20%28single-precision%29))
  (Utilities|FlowControl|Sequence
    (:then_0
      (LocalVariables|SetgX (.x GridXYZ))
      (LocalVariables|SetgY (.y GridXYZ))
      (LocalVariables|SetgZ (.z GridXYZ)))
    (:then_1
      (Utilities|FlowControl|Sequence
        (:then_0
          (LocalVariables|Setradius (Math|Float|Sqrt (+ (Math|Float|Square (LocalVariables|GetgX)) (Math|Float|Square (LocalVariables|GetgY)) (Math|Float|Square (LocalVariables|GetgZ))))))
        (:then_1
          (LocalVariables|Setazimuth (Class|KismetMathLibrary|DegAtan2 (LocalVariables|GetgY) (LocalVariables|GetgX))))
        (:then_2
          (LocalVariables|Setinclination (Class|KismetMathLibrary|DegAcos (/ (LocalVariables|GetgZ) (LocalVariables|Getradius)))))))
    (:then_2
      (return (Utilities|Struct|MakeSphereCoordsStruct SetRadius (LocalVariables|Getazimuth) (LocalVariables|Getinclination))))))