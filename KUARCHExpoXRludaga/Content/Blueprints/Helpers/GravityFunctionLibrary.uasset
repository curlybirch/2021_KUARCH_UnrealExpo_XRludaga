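; Blueprint function library that computes per-frame gravity velocity changes, scaled by delta time and a factor of 100 between metres and centimetres.
; 3DGrav pulls an item toward a source point with inverse-square falloff from G, mass and squared distance.
; 2DGrav applies a constant acceleration toward a source point.
; 1DGrav applies a constant acceleration along the world Z axis, with its sign set by the input.
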(fn 3DGrav
  (params (ItemLocation :type Vector) (3D%20Grav%20Source :type Vector :default "0,0,0.000000") (Big%20G :type Float%20%28single-precision%29) (Mass :type Float%20%28single-precision%29) (DeltaSeconds :type Float%20%28single-precision%29))
  (return (* (Math|Vector|GetUnitDirection(Vector) ItemLocation 3D%20Grav%20Source) (* (* (/ (* Big%20G Mass) (Class|KismetMathLibrary|VectorDistanceSquared 3D%20Grav%20Source ItemLocation)) DeltaSeconds) 1e+02))))

(fn 2DGrav
  (params (ItemLocation :type Vector) (3D%20Grav%20Source :type Vector) (m/sec^2 :type Float%20%28single-precision%29) (Delta%20Seconds :type Float%20%28single-precision%29))
  (return (* (Math|Vector|GetUnitDirection(Vector) ItemLocation 3D%20Grav%20Source) (* (* m/sec^2 Delta%20Seconds) 1e+02))))

(fn 1DGrav
  (params (m/sec^2 :type Float%20%28single-precision%29) (Delta%20Seconds :type Float%20%28single-precision%29))
  (return (Math|Vector|MakeVector 0.0 0.0 (* (* m/sec^2 Delta%20Seconds) 1e+02))))